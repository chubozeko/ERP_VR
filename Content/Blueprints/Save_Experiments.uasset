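; Save_Experiments stores trial definitions and recorded results for two experiments built around exemplars and cue words.
; Each experiment's save function fills its trial list only when empty, then appends that list's fields to shared parallel arrays on every call.
; GetCurrentTrialIndex matches the current trial number and experiment ID to an array index.
; Index-based functions read exemplar and cue data and write exemplar timings and timed responses.
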(fn `Break ETrials`
  (params (ETrials :type "Array of /Game/Blueprints/ETrial Object Reference"))
  (for (_array_element _array_index) ETrials
    (`KismetArrayLibrary.Array_Add` (`self.Trial Indexes`) _array_index)
    (`KismetArrayLibrary.Array_Add` (`self.Trial Numbers`) (`/Game/Blueprints/ETrial.Trial Number` _array_element))
    (`KismetArrayLibrary.Array_Add` (`self.Experiment IDs`) (`/Game/Blueprints/ETrial.Experiment ID` _array_element))
    (`KismetArrayLibrary.Array_Add` (`self.Exemplar Names`) (`/Game/Blueprints/ETrial.Exemplar Name` _array_element))
    (`KismetArrayLibrary.Array_Add` (`self.Exemplar Types`) (`/Game/Blueprints/ETrial.Exemplar Type` _array_element))
    (`KismetArrayLibrary.Array_Add` (`self.Cue Words`) (`/Game/Blueprints/ETrial.Cue Word` _array_element))
    (`KismetArrayLibrary.Array_Add` (`self.Responses`) (`/Game/Blueprints/ETrial.Response` _array_element))
    (`KismetArrayLibrary.Array_Add` (`self.Response Start Times`) (`/Game/Blueprints/ETrial.Response Start Time` _array_element))
    (`KismetArrayLibrary.Array_Add` (`self.Response End Times`) (`/Game/Blueprints/ETrial.Response End Time` _array_element))))

(fn `Get Cue Word with Index`
  (params (Index :type Integer))
  (returns (`Cue Word` :type String))
  (locals (`Current Trial` :type "/Game/Blueprints/ETrial Object Reference"))
  (return (`|GetArrayItem` (`self.Cue Words`) Index)))

(fn `Get Current Trial Index`
  (returns (`Trial Index` :type Integer))
  (locals (`Current Trial` :type "/Game/Blueprints/ETrial Object Reference"))
  (for (_array_element _array_index) (`self.Trial Numbers`)
    (if (and (== _array_element (`self.Current Trial Number`)) (== (`self.Current Experiment ID`) (`|GetArrayItem` (`self.Experiment IDs`) _array_index)))
      (return _array_index))))

(fn `Get Exemplar Name with Index`
  (params (Index :type Integer))
  (returns (`Exemplar Name` :type String))
  (locals (`Current Trial` :type "/Game/Blueprints/ETrial Object Reference"))
  (return (`|GetArrayItem` (`self.Exemplar Names`) Index)))

(fn `Get Exemplar Type with Index`
  (params (Index :type Integer))
  (returns (`Exemplar Type` :type String))
  (locals (`Current Trial` :type "/Game/Blueprints/ETrial Object Reference"))
  (return (`|GetArrayItem` (`self.Exemplar Types`) Index)))

(fn `Save Exemplar Times`
  (params (Index :type Integer) (`Start Time` :type "DateTime Structure") (`End Time` :type "DateTime Structure"))
  (`KismetArrayLibrary.Array_Set` (`self.Exemplar Start Times`) Index `Start Time`)
  (`KismetArrayLibrary.Array_Set` (`self.Exemplar End Times`) Index `End Time`))

(fn `Save Experiment 1 Trials`
  (params (Trials :type "Array of /Game/Blueprints/ExperimentTrial Object Reference"))
  (returns (`New Trials` :type "Array of /Game/Blueprints/ETrial Object Reference") (Length :type Integer))
  (bind _experiment_1_trials (`self.Experiment 1 Trials`))
  (if (`KismetArrayLibrary.Array_IsEmpty` _experiment_1_trials)
    (for _array_element Trials
      (`KismetArrayLibrary.Array_Add` (`self.Experiment 1 Trials`) (`/Game/Blueprints/ExperimentTrial.ETrial` _array_element))))
  (`self.Break ETrials` _experiment_1_trials)
  (return _experiment_1_trials (`KismetArrayLibrary.Array_LastIndex` _experiment_1_trials)))

(fn `Save Experiment 2 Trials`
  (params (Trials :type "Array of /Game/Blueprints/ExperimentTrial Object Reference"))
  (returns (`New Trials` :type "Array of /Game/Blueprints/ETrial Object Reference") (Length :type Integer))
  (bind _experiment_2_trials (`self.Experiment 2 Trials`))
  (if (`KismetArrayLibrary.Array_IsEmpty` _experiment_2_trials)
    (for _array_element Trials
      (`KismetArrayLibrary.Array_Add` (`self.Experiment 2 Trials`) (`/Game/Blueprints/ExperimentTrial.ETrial` _array_element))))
  (`self.Break ETrials` _experiment_2_trials)
  (return _experiment_2_trials (`KismetArrayLibrary.Array_LastIndex` _experiment_2_trials)))

(fn `Save Responses`
  (params (Index :type Integer) (Response :type String) (`Response Start Time` :type "DateTime Structure") (`Response End Time` :type "DateTime Structure"))
  (`KismetArrayLibrary.Array_Set` (`self.Responses`) Index Response)
  (`KismetArrayLibrary.Array_Set` (`self.Response Start Times`) Index `Response Start Time`)
  (`KismetArrayLibrary.Array_Set` (`self.Response End Times`) Index `Response End Time`)
  (return))