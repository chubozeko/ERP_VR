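; ExemplarRoom is a VR viewing room actor that shows exemplar 360 images on a globe.
; SetViewingGlobeMaterial stores the exemplar, applies its material to ViewingGlobe, and rotates the actor to its desired rotation with a 90-degree yaw offset.
; The event graph holds only disconnected debug logic for stepping through Exemplars and printing ratings or laser pointer yaw, none of which runs.
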(event `self.ReceiveBeginPlay`
  ;[0.1562 0.009766 0.009766] !! For DEBUGGING !!
)

(event `Key|P`
  (params (Key :type "Key Structure"))
  ;[0.1562 0.009766 0.009766] !! For DEBUGGING !!
)

(event `Key|O`
  (params (Key :type "Key Structure"))
  ;[0.1562 0.009766 0.009766] !! For DEBUGGING !!
)

(event `Key|L`
  (params (Key :type "Key Structure"))
  ;[0.1562 0.009766 0.009766] !! For DEBUGGING !!
)

(event `Key|G`
  (params (Key :type "Key Structure"))
  ;[0.1562 0.009766 0.009766] !! For DEBUGGING !!
)

(event `Key|B`
  (params (Key :type "Key Structure"))
  ;[0.1562 0.009766 0.009766] !! For DEBUGGING !!
)

(fn `Set Viewing Globe Material`
  (params (`Current Exemplar` :type "/Game/Blueprints/ExemplarObject Object Reference"))
  (bind (_desired_rotation_roll _desired_rotation_pitch _desired_rotation_yaw) (`KismetMathLibrary.BreakRotator` (`/Game/Blueprints/ExemplarObject.Desired Rotation` (`self.Current Exemplar`))))
  (bind _output_get (set `self.Current Exemplar` `Current Exemplar`))
  (bind _material (`/Game/Blueprints/ExemplarObject.Get Material` _output_get))
  (bind _output_get_2 (set `self.360 Image Material` _material))
  (`PrimitiveComponent.SetMaterial` (`self.Viewing Globe`) 0 _output_get_2)
  (`self.K2_SetActorRotation` self (`KismetMathLibrary.MakeRotator` _desired_rotation_roll _desired_rotation_pitch (- _desired_rotation_yaw 90.0)) false))

(fn `UserConstructionScript`)