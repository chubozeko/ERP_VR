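; Save_Experiments stores trial data for two experiments and exports the results to CSV files in the project's Experiments folder.
; Loaded trials are flattened into shared parallel arrays, with the current index found by trial number and experiment ID.
; Index-based setters record exemplar times, responses and category ratings.
; Export writes ratings for experiment 1 or cue-word responses for experiment 2, with timestamps as zero-padded time-of-day strings.
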(fn `Break ETrials`
  (params (ETrials :type "Array of /Game/Blueprints/ETrial Object Reference"))
  (for (_array_element _array_index) ETrials
    (`KismetArrayLibrary.Array_Add` (`self.Trial Indexes`) _array_index)
    (`KismetArrayLibrary.Array_Add` (`self.Trial Numbers`) (`/Game/Blueprints/ETrial.Trial Number` _array_element))
    (`KismetArrayLibrary.Array_Add` (`self.Experiment IDs`) (`/Game/Blueprints/ETrial.Experiment ID` _array_element))
    (`KismetArrayLibrary.Array_Add` (`self.Exemplar Names`) (`/Game/Blueprints/ETrial.Exemplar Name` _array_element))
    (`KismetArrayLibrary.Array_Add` (`self.Exemplar Types`) (`/Game/Blueprints/ETrial.Exemplar Type` _array_element))
    (`KismetArrayLibrary.Array_Add` (`self.Cue Words`) (`/Game/Blueprints/ETrial.Cue Word` _array_element))
    (`KismetArrayLibrary.Array_Add` (`self.Responses`) (`/Game/Blueprints/ETrial.Response` _array_element))
    (`KismetArrayLibrary.Array_Add` (`self.Response Start Times`) (`/Game/Blueprints/ETrial.Response Start Time` _array_element))
    (`KismetArrayLibrary.Array_Add` (`self.Response End Times`) (`/Game/Blueprints/ETrial.Response End Time` _array_element))
    (`KismetArrayLibrary.Array_Add` (`self.Exemplar Start Times`) (`/Game/Blueprints/ETrial.Exemplar Start Time` _array_element))
    (`KismetArrayLibrary.Array_Add` (`self.Exemplar End Times`) (`/Game/Blueprints/ETrial.Exemplar End Time` _array_element))
    (`KismetArrayLibrary.Array_Add` (`self.Selected Categories`) (`/Game/Blueprints/ETrial.Selected Category` _array_element))
    (`KismetArrayLibrary.Array_Add` (`self.Ratings`) (`/Game/Blueprints/ETrial.Rating` _array_element))))

(fn `Get Cue Word with Index`
  (params (Index :type Integer))
  (returns (`Cue Word` :type String))
  (locals (`Current Trial` :type "/Game/Blueprints/ETrial Object Reference"))
  (return (`|GetArrayItem` (`self.Cue Words`) Index)))

(fn `Get Current Trial Index`
  (returns (`Trial Index` :type Integer))
  (locals (`Current Trial` :type "/Game/Blueprints/ETrial Object Reference"))
  (for (_array_element _array_index) (`self.Trial Numbers`)
    (if (and (== _array_element (`self.Current Trial Number`)) (== (`self.Current Experiment ID`) (`|GetArrayItem` (`self.Experiment IDs`) _array_index)))
      (return _array_index))))

(fn `Get Exemplar Name with Index`
  (params (Index :type Integer))
  (returns (`Exemplar Name` :type String))
  (locals (`Current Trial` :type "/Game/Blueprints/ETrial Object Reference"))
  (return (`|GetArrayItem` (`self.Exemplar Names`) Index)))

(fn `Get Exemplar Type with Index`
  (params (Index :type Integer))
  (returns (`Exemplar Type` :type String))
  (locals (`Current Trial` :type "/Game/Blueprints/ETrial Object Reference"))
  (return (`|GetArrayItem` (`self.Exemplar Types`) Index)))

(fn `Parse DateTime to Full Time String`
  (params (`Date Time` :type "DateTime Structure"))
  (returns (`Full Time String` :type String))
  (bind (_year _month _day _hour _minute _second _millisecond) (`KismetMathLibrary.BreakDateTime` `Date Time`))
  (bind _int_string (`self.Parse Int to String` _hour))
  (bind _int_string_2 (`self.Parse Int to String` _minute))
  (bind _int_string_3 (`self.Parse Int to String` _second))
  (bind _int_string_4 (`self.Parse Int to String` _millisecond))
  (bind _int_string_5 (`self.Parse Int to String` 0))
  (return (`KismetStringLibrary.Concat_StrStr` _int_string ":" _int_string_2 ":" _int_string_3 ":" _int_string_4 ":" _int_string_5)))

(fn `Parse Int to String`
  (params (Int :type Integer))
  (returns (`Int String` :type String))
  (locals (`New Int` :type String))
  (bind _returnvalue (`KismetStringLibrary.Conv_IntToString` Int))
  (if (< Int 10)
    (set `local.New Int` (`KismetStringLibrary.Concat_StrStr` "0" _returnvalue))
    (else
      (set `local.New Int` _returnvalue)))
  (return (`local.New Int`)))

(fn `Save Exemplar Times`
  (params (Index :type Integer) (`Start Time` :type "DateTime Structure") (`End Time` :type "DateTime Structure"))
  (`KismetArrayLibrary.Array_Set` (`self.Exemplar Start Times`) Index `Start Time`)
  (`KismetArrayLibrary.Array_Set` (`self.Exemplar End Times`) Index `End Time`)
  (return))

(fn `Save Experiment 1 Trials`
  (params (Trials :type "Array of /Game/Blueprints/ExperimentTrial Object Reference"))
  (returns (`New Trials` :type "Array of /Game/Blueprints/ETrial Object Reference") (Length :type Integer))
  (bind _experiment_1_trials (`self.Experiment 1 Trials`))
  (if (`KismetArrayLibrary.Array_IsEmpty` _experiment_1_trials)
    (for _array_element Trials
      (`KismetArrayLibrary.Array_Add` (`self.Experiment 1 Trials`) (`/Game/Blueprints/ExperimentTrial.ETrial` _array_element))))
  (`self.Break ETrials` _experiment_1_trials)
  (return _experiment_1_trials (`KismetArrayLibrary.Array_LastIndex` _experiment_1_trials)))

(fn `Save Experiment 2 Trials`
  (params (Trials :type "Array of /Game/Blueprints/ExperimentTrial Object Reference"))
  (returns (`New Trials` :type "Array of /Game/Blueprints/ETrial Object Reference") (Length :type Integer))
  (bind _experiment_2_trials (`self.Experiment 2 Trials`))
  (if (`KismetArrayLibrary.Array_IsEmpty` _experiment_2_trials)
    (for _array_element Trials
      (`KismetArrayLibrary.Array_Add` (`self.Experiment 2 Trials`) (`/Game/Blueprints/ExperimentTrial.ETrial` _array_element))))
  (`self.Break ETrials` _experiment_2_trials)
  (return _experiment_2_trials (`KismetArrayLibrary.Array_LastIndex` _experiment_2_trials)))

(fn `Save Ratings`
  (params (Index :type Integer) (Category :type String) (Rating :type Integer))
  (`KismetArrayLibrary.Array_Set` (`self.Selected Categories`) Index Category)
  (`KismetArrayLibrary.Array_Set` (`self.Ratings`) Index Rating)
  (return))

(fn `Save Responses`
  (params (Index :type Integer) (Response :type String) (`Response Start Time` :type "DateTime Structure") (`Response End Time` :type "DateTime Structure"))
  (`KismetArrayLibrary.Array_Set` (`self.Responses`) Index Response)
  (`KismetArrayLibrary.Array_Set` (`self.Response Start Times`) Index `Response Start Time`)
  (`KismetArrayLibrary.Array_Set` (`self.Response End Times`) Index `Response End Time`)
  (return))

(fn `Save Trials to CSV`
  (params (`CSV File Name` :type String))
  (locals (`Save Text (Exp 1)` :type "Array of String") (`Save Text (Exp 2)` :type "Array of String"))
  (switch `int` (`self.Current Experiment ID`)
    (:`1`
      (for (_ _array_index) (`self.Trial Indexes`)
        (bind _full_time_string (`self.Parse DateTime to Full Time String` (`|GetArrayItem` (`self.Exemplar Start Times`) _array_index)))
        (bind _full_time_string_2 (`self.Parse DateTime to Full Time String` (`|GetArrayItem` (`self.Exemplar End Times`) _array_index)))
        (`KismetArrayLibrary.Array_Add` (`local.Save Text (Exp 1)`) (`KismetStringLibrary.Concat_StrStr` (`KismetStringLibrary.Conv_IntToString` (`|GetArrayItem` (`self.Trial Numbers`) _array_index)) "," (`KismetStringLibrary.Conv_IntToString` (`|GetArrayItem` (`self.Experiment IDs`) _array_index)) "," (`|GetArrayItem` (`self.Exemplar Names`) _array_index) "," (`|GetArrayItem` (`self.Exemplar Types`) _array_index) "," _full_time_string "," _full_time_string_2 "," (`|GetArrayItem` (`self.Selected Categories`) _array_index) "," (`KismetStringLibrary.Conv_IntToString` (`|GetArrayItem` (`self.Ratings`) _array_index)))))
      (`BPFL_TextFileManager.SaveArrayText` (`KismetStringLibrary.Concat_StrStr` (`KismetSystemLibrary.GetProjectDirectory`) "\\Experiments\\") (`local.CSV File Name`) (`local.Save Text (Exp 1)`)))
    (:`2`
      (for (_ _array_index_2) (`self.Trial Indexes`)
        (bind _full_time_string_3 (`self.Parse DateTime to Full Time String` (`|GetArrayItem` (`self.Exemplar Start Times`) _array_index_2)))
        (bind _full_time_string_4 (`self.Parse DateTime to Full Time String` (`|GetArrayItem` (`self.Exemplar End Times`) _array_index_2)))
        (bind _full_time_string_5 (`self.Parse DateTime to Full Time String` (`|GetArrayItem` (`self.Response Start Times`) _array_index_2)))
        (bind _full_time_string_6 (`self.Parse DateTime to Full Time String` (`|GetArrayItem` (`self.Response End Times`) _array_index_2)))
        (`KismetArrayLibrary.Array_Add` (`local.Save Text (Exp 2)`) (`KismetStringLibrary.Concat_StrStr` (`KismetStringLibrary.Conv_IntToString` (`|GetArrayItem` (`self.Trial Numbers`) _array_index_2)) "," (`KismetStringLibrary.Conv_IntToString` (`|GetArrayItem` (`self.Experiment IDs`) _array_index_2)) "," (`|GetArrayItem` (`self.Exemplar Names`) _array_index_2) "," (`|GetArrayItem` (`self.Exemplar Types`) _array_index_2) "," _full_time_string_3 "," _full_time_string_4 "," (`|GetArrayItem` (`self.Cue Words`) _array_index_2) "," (`|GetArrayItem` (`self.Responses`) _array_index_2) "," _full_time_string_5 "," _full_time_string_6)))
      (`BPFL_TextFileManager.SaveArrayText` (`KismetStringLibrary.Concat_StrStr` (`KismetSystemLibrary.GetProjectDirectory`) "\\Experiments\\") (`local.CSV File Name`) (`local.Save Text (Exp 2)`)))))