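; Game instance for experiments that holds the experiment type and the trial number to run, both set through an Initialize event.
; It builds and stores timestamped names: a save slot name suffixed with the experiment type and a CSV file name for trials.
; Helper functions format the current date and time as a compact, zero-padded string shared by both names.
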(event `Event Initialize`
  (params (Type :type Integer) (`Trial Nr` :type Integer))
  (set `self.Experiment Type` Type)
  (set `self.Trial Number to Run` `Trial Nr`))

(fn `Generate Exp File Name`
  (returns (`File Name` :type String))
  (bind _new_dt_string (`self.Parse DateTime to String` (`KismetMathLibrary.Now`)))
  (bind _output_get (set `self.Experiment File Name` (`KismetStringLibrary.Concat_StrStr` "Trials_" _new_dt_string ".csv")))
  (return _output_get))

(fn `Generate Save Slot Name`
  (returns (`Save Slot Name` :type String))
  (bind _new_dt_string (`self.Parse DateTime to String` (`KismetMathLibrary.Now`)))
  (bind _output_get (set `self.Save Slot Name` (`KismetStringLibrary.Concat_StrStr` _new_dt_string "_Exp" (`KismetStringLibrary.Conv_IntToString` (`self.Experiment Type`)))))
  (return _output_get))

(fn `Parse DateTime to String`
  (params (`Date Time` :type "DateTime Structure"))
  (returns (`New DT String` :type String))
  (bind (_year _month _day _hour _minute _second) (`KismetMathLibrary.BreakDateTime` `Date Time`))
  (bind _int_string (`self.Parse Int to String` _month))
  (bind _int_string_2 (`self.Parse Int to String` _day))
  (bind _int_string_3 (`self.Parse Int to String` _hour))
  (bind _int_string_4 (`self.Parse Int to String` _minute))
  (bind _int_string_5 (`self.Parse Int to String` _second))
  (return (`KismetStringLibrary.Concat_StrStr` (`KismetStringLibrary.Conv_IntToString` _year) _int_string _int_string_2 "_" _int_string_3 _int_string_4 _int_string_5)))

(fn `Parse Int to String`
  (params (Int :type Integer))
  (returns (`Int String` :type String))
  (locals (`New Int` :type String))
  (bind _returnvalue (`KismetStringLibrary.Conv_IntToString` Int))
  (if (< Int 10)
    (set `local.New Int` (`KismetStringLibrary.Concat_StrStr` "0" _returnvalue))
    (else
      (set `local.New Int` _returnvalue)))
  (return (`local.New Int`)))