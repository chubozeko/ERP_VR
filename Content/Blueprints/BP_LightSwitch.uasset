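; BP_LightSwitch is an interactable wall switch that toggles the visibility of an array of point lights.
; Entering its box caches the BP_FPS_Character and shows the interact text, which hides again on exit.
; InteractwithObject acts only if that character is looking at the switch, flipping each light individually and rotating the switch mesh by the last light's new state.
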(event `self.InteractWithObject`
  (bind _switch (`self.Switch`))
  ;[1 0.9439 0.3421] Light Switch
  (if (== (`/Game/Blueprints/BP_FPS_Character.ObjectLookingAt` (stale `self.Box.OnComponentBeginOverlap` _asbp_fps_character)) self)
    (for _array_element (`self.Light`)
      (bind _pointlightcomponent (`PointLight.PointLightComponent` _array_element))
      (bind _bhiddeningame (`SceneComponent.bHiddenInGame` _pointlightcomponent))
      (if _bhiddeningame
        (`SceneComponent.SetHiddenInGame` _pointlightcomponent false false)
        (else
          (`SceneComponent.SetHiddenInGame` _pointlightcomponent true false))))
    (if _bhiddeningame
      (`SceneComponent.K2_AddLocalRotation` _switch (struct :`Roll` -20.0) false false)
      (else
        (`SceneComponent.K2_AddLocalRotation` _switch (struct :`Roll` 20.0) false false)))))

(event `self.Box.OnComponentBeginOverlap`
  (params (OverlappedComponent :type "PrimitiveComponent Object Reference") (OtherActor :type "Actor Object Reference") (OtherComp :type "PrimitiveComponent Object Reference") (OtherBodyIndex :type Integer) (bFromSweep :type Boolean) (SweepResult :type "HitResult Structure (by ref)"))
  (bind _asbp_fps_character (cast `/Game/Blueprints/BP_FPS_Character` OtherActor))
  (`SceneComponent.SetHiddenInGame` (`self.InteractText`) false false))

(event `self.Box.OnComponentEndOverlap`
  (params (OverlappedComponent :type "PrimitiveComponent Object Reference") (OtherActor :type "Actor Object Reference") (OtherComp :type "PrimitiveComponent Object Reference") (OtherBodyIndex :type Integer))
  (cast `/Game/Blueprints/BP_FPS_Character` OtherActor)
  (`SceneComponent.SetHiddenInGame` (`self.InteractText`) true false))

(fn `UserConstructionScript`
  (`parent.UserConstructionScript`))