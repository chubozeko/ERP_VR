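; ExperimentTrial holds the data for one trial of a psychology-style experiment: trial number, exemplar, experiment type, cue word and player response.
; Construction sets crosshair, exemplar, fade and cue-word intervals, with a shorter set left unconnected.
; InitializeTrial stores its inputs, forwards them to an ETrial object and returns itself.
; Helpers record the response, derive response time from start and end timestamps, and return the exemplar type as text.
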(fn `Calculate Response Time`
  (bind (_year _month _day _hour _minute _second _millisecond) (`KismetMathLibrary.BreakDateTime` (`self.Response Start Time`)))
  (bind (_year_2 _month_2 _day_2 _hour_2 _minute_2 _second_2 _millisecond_2) (`KismetMathLibrary.BreakDateTime` (`self.Response End Time`)))
  (set `self.Response Timespan` (`KismetMathLibrary.MakeTimespan` 0 (- _hour_2 _hour) (- _minute_2 _minute) (- _second_2 _second) (- _millisecond_2 _millisecond))))

(fn `Create ETrial Instance`
  (returns (`New ETrial` :type "/Game/Blueprints/ETrial Object Reference"))
  (bind _output_get (set `self.ETrial` null))
  (bind _trial (`/Game/Blueprints/ETrial.Initialize Trial` _output_get (`self.Trial Number`) (`self.Exemplar Object`) (`self.Experiment Type`) (`self.Cue Word`)))
  (return _trial))

(fn `Get Exemplar Type`
  (returns (`Exemplar Type` :type String))
  (return (`|GetEnumeratorNameAsString` (`/Game/Blueprints/ExemplarObject.Exemplar Type` (`self.Exemplar Object`)))))

(fn `Initialize Trial`
  (params (`Trial Number` :type Integer) (Exemplar :type "/Game/Blueprints/ExemplarObject Object Reference") (`Experiment Type` :type "/Game/Scripts/ExperimentType Enum" :default "NewEnumerator0") (`Cue Word` :type String))
  (returns (Trial :type "/Game/Blueprints/ExperimentTrial Object Reference"))
  (bind _output_get (set `self.Trial Number` `Trial Number`))
  (bind _output_get_2 (set `self.Exemplar Object` Exemplar))
  (bind _output_get_3 (set `self.Experiment Type` `Experiment Type`))
  (bind _output_get_4 (set `self.Cue Word` `Cue Word`))
  (`/Game/Blueprints/ETrial.Initialize Trial` (`self.ETrial`) _output_get _output_get_2 _output_get_3 _output_get_4)
  (return self))

(fn `Set Player Response`
  (params (Response :type String))
  (set `self.Player Response` Response))

(fn `UserConstructionScript`
  ;[0.2812 0.09417 0.349 0.5 14] Initialize Intervals
  (set `self.Crosshair Interval` 2000.0)
  (set `self.Exemplar Interval` 5000.0)
  (set `self.Fade Interval` 1000.0)
  (set `self.Cue Word Interval` 3000.0))