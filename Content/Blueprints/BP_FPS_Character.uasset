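; First-person player character for a trial-based experiment game, handling look input, interaction, HUD creation, CSV export and quitting.
; Save Session stores data from whichever experiment controller is present in a Save_Experiments slot, advancing or resetting trial progress and updating the game instance.
; Load Session pushes saved experiment and trial state back into the supplied controller.
; The line trace that sets the interact target is disconnected, as is the experiment-update binding.
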(event `self.ReceiveBeginPlay`
  (bind _asgi_experiments (cast `/Game/Blueprints/GI_Experiments` (`GameplayStatics.GetGameInstance`)))
  (bind _output_get (set `self.GameInstance` _asgi_experiments))
  (`/Game/Blueprints/GI_Experiments.Event Initialize` _output_get 0 0)
  (bind _returnvalue (`|CreateWidget` "/Game/UI/FPS_HUD.FPS_HUD_C"))
  (`UserWidget.AddToViewport` _returnvalue 0))

(event `UpdateExperimentProps_Event`
  (params (Type :type Integer) (Trial :type "/Game/Blueprints/ExperimentTrial Object Reference"))
  (bind _gameinstance (`self.GameInstance`))
  (`/Game/Blueprints/GI_Experiments.Event Initialize` _gameinstance Type 0)
  (set `self.Current Experiment Type` (`/Game/Blueprints/GI_Experiments.Experiment Type` _gameinstance)))

(event `self.ReceiveTick`
  (params (DeltaSeconds :type "Float (single-precision)")))

(event `InputAxis|LookUp/LookDown`
  (params (AxisValue :type "Float (single-precision)"))
  ;[1 0.3157 0.8759] Camera Movement Controls
  (`self.AddControllerPitchInput` (`KismetMathLibrary.FClamp` AxisValue -1.0)))

(event `InputAxis|LookRight/LookLeft`
  (params (AxisValue :type "Float (single-precision)"))
  ;[1 0.3157 0.8759] Camera Movement Controls
  (`self.AddControllerYawInput` (`KismetMathLibrary.FClamp` AxisValue -1.0)))

(event `InputAction|Interact`
  (params (Key :type "Key Structure"))
  ;[1 1 1] Interact
  (:`Pressed`
    (bind _asmaster_interact (cast `/Game/Blueprints/Master_Interact` (`self.ObjectLookingAt`)))
    (`/Game/Blueprints/Master_Interact.InteractWithObject` _asmaster_interact)))

(event `InputAction|SaveCSV`
  (params (Key :type "Key Structure"))
  (:`Pressed`
    (bind _assave_experiments (cast `/Game/Blueprints/Save_Experiments` (`self.Save REF`)))
    (bind _file_name (`/Game/Blueprints/GI_Experiments.Generate Exp File Name` (`self.GameInstance`)))
    (`/Game/Blueprints/Save_Experiments.Save Trials to CSV` _assave_experiments _file_name)
    (`KismetSystemLibrary.PrintString` (`KismetStringLibrary.Concat_StrStr` "Saved as " _file_name))))

(event `InputAction|Quit`
  (params (Key :type "Key Structure"))
  (:`Pressed`
    (`KismetSystemLibrary.QuitGame` null "Quit")))

(fn `Load Session`
  (params (Controller :type "Actor Object Reference") (`Slot Name` :type String))
  (locals (`Save Exp` :type "/Game/Blueprints/Save_Experiments Object Reference"))
  (bind _returnvalue (`GameplayStatics.DoesSaveGameExist` `Slot Name`))
  (if _returnvalue
    (bind _returnvalue_2 (`GameplayStatics.LoadGameFromSlot` (`local.Slot Name`)))
    (bind _output_get (set `self.Save REF` _returnvalue_2))
    (bind _assave_experiments (cast `/Game/Blueprints/Save_Experiments` _output_get))
    (set `self.SG Save Experiments` _assave_experiments)
    (cast `/Game/Blueprints/ERP_Controller` Controller
      (:`CastFailed`
        (bind _asexperiment_controller (cast `/Game/Blueprints/ExperimentController` Controller)
          (:`then`
            (bind _current_experiment_id (`/Game/Blueprints/Save_Experiments.Current Experiment ID` _assave_experiments))
            ;[0 0.4948 0.02766 0.5 14] Set values in ExperimentController from SaveGame
            (switch `int` _current_experiment_id
              (:`1`
                (set `/Game/Blueprints/ExperimentController.Experiment Type` "NewEnumerator0" _asexperiment_controller))
              (:`2`
                (set `/Game/Blueprints/ExperimentController.Experiment Type` "NewEnumerator1" _asexperiment_controller)))
            (set `/Game/Blueprints/ExperimentController.Current Trial Number` (`/Game/Blueprints/Save_Experiments.Current Trial Number` _assave_experiments) _asexperiment_controller))
          (:`CastFailed`
            (bind _asetrial_controller (cast `/Game/Blueprints/ETrialController` Controller))
            ;[0 0.4948 0.03043 0.5] Set values in ETrialController from SaveGame
            (set `/Game/Blueprints/ETrialController.Experiment ID` _current_experiment_id _asetrial_controller)
            (bind _trial_index (`/Game/Blueprints/Save_Experiments.Get Current Trial Index` _assave_experiments))
            (bind _output_get_2 (set `/Game/Blueprints/ETrialController.Current Trial Index` _trial_index _asetrial_controller))
            (bind _exemplar_type (`/Game/Blueprints/Save_Experiments.Get Exemplar Type with Index` _assave_experiments _output_get_2))
            (set `/Game/Blueprints/ETrialController.Exemplar Type` _exemplar_type _asetrial_controller)
            (bind _cue_word (`/Game/Blueprints/Save_Experiments.Get Cue Word with Index` _assave_experiments _output_get_2))
            (set `/Game/Blueprints/ETrialController.Cue Word` _cue_word _asetrial_controller)))))))

(fn `Save Session`
  (params (`Slot Name` :type String))
  (bind _gameinstance (`self.GameInstance`))
  (bind _sg_save_experiments (`self.SG Save Experiments`))
  (bind _sg_save_experiments_2 (`self.SG Save Experiments`))
  (bind _gameinstance_2 (`self.GameInstance`))
  (bind _returnvalue (`GameplayStatics.DoesSaveGameExist` `Slot Name`))
  (if _returnvalue
    (bind _returnvalue_2 (`GameplayStatics.LoadGameFromSlot` (`local.Slot Name`)))
    (set `self.Save REF` _returnvalue_2)
    (else
      (bind _returnvalue_3 (`GameplayStatics.CreateSaveGameObject` "/Game/Blueprints/Save_Experiments.Save_Experiments_C"))
      (set `self.Save REF` _returnvalue_3)))
  (bind _assave_experiments (cast `/Game/Blueprints/Save_Experiments` (`self.Save REF`)))
  (set `self.SG Save Experiments` _assave_experiments)
  (bind _returnvalue_4 (`GameplayStatics.GetActorOfClass` "/Game/Blueprints/ERP_Controller.ERP_Controller_C"))
  (if (`KismetSystemLibrary.IsValid` _returnvalue_4)
    (bind _experiment_id (`/Game/Blueprints/ERP_Controller.Experiment ID` _returnvalue_4))
    (switch `int` _experiment_id
      (:`1`
        ;[0 0.3185 0.01938 0.502 14] Save values from ERP Controller (Home)
        (bind (_new_trials _length) (`/Game/Blueprints/Save_Experiments.Save Experiment 1 Trials` _assave_experiments (`/Game/Blueprints/ERP_Controller.Experiment 1 Trials` _returnvalue_4))))
      (:`2`
        (bind (_new_trials_2 _length_2) (`/Game/Blueprints/Save_Experiments.Save Experiment 2 Trials` _assave_experiments (`/Game/Blueprints/ERP_Controller.Experiment 2 Trials` _returnvalue_4)))))
    (bind _output_get (set `/Game/Blueprints/Save_Experiments.Current Experiment ID` _experiment_id _assave_experiments))
    (switch `int` _output_get
      (:`1`
        (bind _output_get_2 (set `/Game/Blueprints/Save_Experiments.Current Trial Number` (`/Game/Blueprints/ETrial.Trial Number` (`|GetArrayItem` _new_trials)) _sg_save_experiments_2))
        (set `/Game/Blueprints/Save_Experiments.Last Trial Number` _length _sg_save_experiments_2)
        (set `/Game/Blueprints/GI_Experiments.Trial Number to Run` _output_get_2 _gameinstance_2))
      (:`2`
        (bind _output_get_3 (set `/Game/Blueprints/Save_Experiments.Current Trial Number` (`/Game/Blueprints/ETrial.Trial Number` (`|GetArrayItem` _new_trials_2)) _sg_save_experiments))
        (set `/Game/Blueprints/Save_Experiments.Last Trial Number` _length_2 _sg_save_experiments)
        (set `/Game/Blueprints/GI_Experiments.Trial Number to Run` _output_get_3 _gameinstance_2)))
    (set `/Game/Blueprints/GI_Experiments.Experiment Type` _output_get _gameinstance_2)
    (`GameplayStatics.SaveGameToSlot` (`self.Save REF`) (`local.Slot Name`) :!label _label)
    (else
      (bind _returnvalue_5 (`GameplayStatics.GetActorOfClass` "/Game/Blueprints/ExperimentController.ExperimentController_C"))
      (if (`KismetSystemLibrary.IsValid` _returnvalue_5)
        ;[0 0.3185 0.01938 0.502 14] Save values from ExperimentController (Experiment_1 / Experiment_2)
        (`/Game/Blueprints/Save_Experiments.Save Exemplar Times` _assave_experiments (`/Game/Blueprints/Save_Experiments.Current Trial Number` _assave_experiments) (`/Game/Blueprints/ExperimentController.Exemplar Start Time` _returnvalue_5) (`/Game/Blueprints/ExperimentController.Exemplar End Time` _returnvalue_5))
        (goto _label)
        (else
          (bind _returnvalue_6 (`GameplayStatics.GetActorOfClass` "/Game/Blueprints/ETrialController.ETrialController_C"))
          (if (`KismetSystemLibrary.IsValid` _returnvalue_6)
            ;[0 0.3185 0.01938 0.502 14] Save values from ETrialController (Experiment_Trial) and increment Current Trial Number
            (bind _trial_index (`/Game/Blueprints/Save_Experiments.Get Current Trial Index` _assave_experiments))
            (`/Game/Blueprints/Save_Experiments.Save Responses` _assave_experiments _trial_index (`/Game/Blueprints/ETrialController.Response` _returnvalue_6) (`/Game/Blueprints/ETrialController.Response Start Time` _returnvalue_6) (`/Game/Blueprints/ETrialController.Response End Time` _returnvalue_6))
            (bind _result (`/Engine/EditorBlueprintResources/StandardMacros.IncrementInt` (`/Game/Blueprints/Save_Experiments.Current Trial Number` _assave_experiments))
              (:`  `
                (if (<= _result (`/Game/Blueprints/Save_Experiments.Last Trial Number` _assave_experiments))
                  (bind _output_get_4 (set `/Game/Blueprints/Save_Experiments.Current Trial Number` _result _assave_experiments))
                  (set `/Game/Blueprints/GI_Experiments.Trial Number to Run` _output_get_4 _gameinstance)
                  (goto _label)
                  (else
                    (set `/Game/Blueprints/Save_Experiments.Current Trial Number` 0 _assave_experiments)
                    (set `/Game/Blueprints/Save_Experiments.Current Experiment ID` 0 _assave_experiments)
                    (set `/Game/Blueprints/GI_Experiments.Trial Number to Run` 0 _gameinstance)
                    (goto _label)))))))))))

(fn `Unset Room Movement`
  (returns (Character :type "/Game/Blueprints/BP_FPS_Character Object Reference"))
  (set `self.MoveToExemplarRoom` false)
  (set `self.MoveToLobbyOffice` false)
  (set `self.MoveToBlackRoom` false)
  (return self))

(fn `UserConstructionScript`)