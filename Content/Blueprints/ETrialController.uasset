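; Runs the response screen of an experiment trial, asking a GOOD/BAD or YES/NO question based on ExperimentID.
; BeginPlay loads the player's session, shows the question, then fades in via Level Sequences and starts response timing.
; Tick polls for selected, looked-at ScreenButtons, though ReturnToLobby is only checked inside the Continue branch.
; Answers record response and end time, save the session, then offer the next trial or, when none remain, the lobby.
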(event `self.ReceiveBeginPlay`
  (`self.Invisible Scene`)
  (`KismetSystemLibrary.Delay` 0.2)
  (bind _asbp_fps_character (cast `/Game/Blueprints/BP_FPS_Character` (`GameplayStatics.GetPlayerCharacter` 0)))
  (bind _output_get (set `self.As BP FPS Character` _asbp_fps_character))
  (bind _gameinstance (`/Game/Blueprints/BP_FPS_Character.GameInstance` _output_get))
  (`/Game/Blueprints/BP_FPS_Character.Load Session` _output_get self (`/Game/Blueprints/GI_Experiments.Save Slot Name` _gameinstance))
  (switch `int` (`self.Experiment ID`)
    (:`1`
      (`self.View Experiment 1 Question`))
    (:`2`
      (`self.View Experiment 2 Question`)))
  (`self.K2_SetActorLocation` (`self.Menu Panel`) (0.0 1085.0 150.0) false true)
  (bind _interval_in_seconds (`self.Convert Interval to Seconds` (`/Game/Blueprints/GI_Experiments.Fade Interval` _gameinstance))) ; Fade Interval
  (`KismetSystemLibrary.Delay` _interval_in_seconds)
  (`self.FadeIntoScene`)
  (set `self.Response Start Time` (`KismetMathLibrary.Now`)))

(event `self.ReceiveTick`
  (params (DeltaSeconds :type "Float (single-precision)"))
  (bind _continue (`self.Continue`))
  (bind _return_to_lobby (`self.Return to Lobby`))
  ;[1 1 1] Check for Object being Looked at
  (for _array_element (`self.Response Buttons`)
    (bind _screenbutton_object (`self.Get Object Looking At As ScreenButton`))
    (if (and (== _screenbutton_object _array_element) (`/Game/Blueprints/ScreenButton.IsSelected` _array_element))
      (`self.Execute Button Function` _array_element)
      (set `/Game/Blueprints/ScreenButton.IsSelected` false _array_element)))
  (bind _screenbutton_object_2 (`self.Get Object Looking At As ScreenButton`))
  (if (and (== _screenbutton_object_2 _continue) (`/Game/Blueprints/ScreenButton.IsSelected` _continue))
    (`self.Execute Button Function` _continue)
    (set `/Game/Blueprints/ScreenButton.IsSelected` false _continue)
    (bind _screenbutton_object_3 (`self.Get Object Looking At As ScreenButton`))
    (if (and (== _screenbutton_object_3 _return_to_lobby) (`/Game/Blueprints/ScreenButton.IsSelected` _return_to_lobby))
      (`self.Execute Button Function` _return_to_lobby)
      (set `/Game/Blueprints/ScreenButton.IsSelected` false _return_to_lobby)
      (for _array_element_2 (`self.End Sessions`)
        (bind _screenbutton_object_4 (`self.Get Object Looking At As ScreenButton`))
        (if (and (== _screenbutton_object_4 _array_element_2) (`/Game/Blueprints/ScreenButton.IsSelected` _array_element_2))
          (`self.Execute Button Function` _array_element_2)
          (set `/Game/Blueprints/ScreenButton.IsSelected` false _array_element_2))))))

(event `View Experiment 1 Question`
  (bind _question (`self.Question`))
  (bind _answer_l (`self.Answer L`))
  (bind _answer_r (`self.Answer R`))
  (bind _crosshair (`self.Crosshair`))
  ;[0.06663 0.05448 0.2918 0.749 14] View Experiment 1 Question
  (`TextRenderComponent.K2_SetText` (`TextRenderActor.TextRender` _crosshair) (`KismetTextLibrary.Conv_StringToText` "+"))
  (`self.SetActorHiddenInGame` _crosshair false)
  (`TextRenderComponent.K2_SetText` (`TextRenderActor.TextRender` _answer_l) (`KismetTextLibrary.Conv_StringToText` "GOOD"))
  (`self.SetActorHiddenInGame` _answer_l false)
  (`TextRenderComponent.K2_SetText` (`TextRenderActor.TextRender` _answer_r) (`KismetTextLibrary.Conv_StringToText` "BAD"))
  (`self.SetActorHiddenInGame` _answer_r false)
  (`TextRenderComponent.K2_SetText` (`TextRenderActor.TextRender` _question) (`KismetTextLibrary.Conv_StringToText` (`KismetStringLibrary.Concat_StrStr` "Was that a GOOD or BAD depiction of a/an " (`self.Exemplar Type`) "?")))
  (`self.SetActorHiddenInGame` _question false))

(event `View Experiment 2 Question`
  (bind _question (`self.Question`))
  (bind _crosshair (`self.Crosshair`))
  (bind _answer_l (`self.Answer L`))
  (bind _answer_r (`self.Answer R`))
  ;[0.06667 0.0549 0.2902 0.749 14] View Experiment 2 Question
  (`TextRenderComponent.K2_SetText` (`TextRenderActor.TextRender` _crosshair) (`KismetTextLibrary.Conv_StringToText` "+"))
  (`self.SetActorHiddenInGame` _crosshair false)
  (`TextRenderComponent.K2_SetText` (`TextRenderActor.TextRender` _answer_l) (`KismetTextLibrary.Conv_StringToText` "YES"))
  (`self.SetActorHiddenInGame` _answer_l false)
  (`TextRenderComponent.K2_SetText` (`TextRenderActor.TextRender` _answer_r) (`KismetTextLibrary.Conv_StringToText` "NO"))
  (`self.SetActorHiddenInGame` _answer_r false)
  (`TextRenderComponent.K2_SetText` (`TextRenderActor.TextRender` _question) (`KismetTextLibrary.Conv_StringToText` (`KismetStringLibrary.Concat_StrStr` "Do you think the Cue Word \"" (`self.Cue Word`) "\" matched the given scene?")))
  (`self.SetActorHiddenInGame` _question false))

(event `View Experiment Complete`
  (bind _menu_panel (`self.Menu Panel`))
  (bind _continue (`self.Continue`))
  (bind _return_to_lobby (`self.Return to Lobby`))
  ;[0.06663 0.05448 0.2918 0.749 14] View Experiment Trial Complete
  (`self.SetActorHiddenInGame` (`self.Crosshair`) true)
  (`self.SetActorHiddenInGame` (`self.Answer L`) true)
  (`self.SetActorHiddenInGame` (`self.Answer R`) true)
  (`self.SetActorHiddenInGame` (`self.Question`) true)
  (`self.SetActorHiddenInGame` (`self.Trial Complete`) false)
  (for _array_element (`self.Response Buttons`)
    (`self.SetActorHiddenInGame` _array_element true))
  (switch `int` (`/Game/Blueprints/GI_Experiments.Trial Number to Run` (`/Game/Blueprints/BP_FPS_Character.GameInstance` (`self.As BP FPS Character`)))
    (:`Default`
      (`self.SetActorHiddenInGame` _continue false)
      (`self.SetActorHiddenInGame` _return_to_lobby true)
      (`self.K2_SetActorLocation` _menu_panel (-400.0 1085.0 150.0) false true))
    (:`0`
      (`self.SetActorHiddenInGame` _continue true)
      (`self.SetActorHiddenInGame` _return_to_lobby false)
      (`self.K2_SetActorLocation` _menu_panel (400.0 1085.0 150.0) false true))))

(fn `Convert Interval to Seconds`
  (params (`Interval in Milliseconds` :type "Float (double-precision)"))
  (returns (`Interval in Seconds` :type "Float (double-precision)"))
  (return (`KismetMathLibrary.Conv_IntToDouble` (/ `Interval in Milliseconds` 1000))))

(fn `Execute Button Function`
  (params (Button :type "/Game/Blueprints/ScreenButton Object Reference"))
  (bind _as_bp_fps_character (`self.As BP FPS Character`))
  (bind _experiment_id (`self.Experiment ID`))
  (switch `string` (`/Game/Blueprints/ScreenButton.Button Function` Button)
    (:`AnswerPositive`
      (switch `int` _experiment_id
        (:`1`
          (set `self.Response` "GOOD"))
        (:`2`
          (set `self.Response` "YES")))
      (set `self.Response End Time` (`KismetMathLibrary.Now`) :!label _label)
      (`/Game/Blueprints/BP_FPS_Character.Save Session` _as_bp_fps_character (`/Game/Blueprints/GI_Experiments.Save Slot Name` (`/Game/Blueprints/BP_FPS_Character.GameInstance` _as_bp_fps_character)))
      (`self.View Experiment Complete`))
    (:`AnswerNegative`
      (switch `int` _experiment_id
        (:`1`
          (set `self.Response` "BAD")
          (goto _label))
        (:`2`
          (set `self.Response` "NO")
          (goto _label))))
    (:`ContinueToNextTrial`
      (`self.FadeToBlack`)
      (`self.Invisible Scene`)
      (switch `int` (`self.Experiment ID`)
        (:`1`
          (`GameplayStatics.OpenLevelBySoftObjectPtr` "/Game/Levels/Experiment_1.Experiment_1"))
        (:`2`
          (`GameplayStatics.OpenLevelBySoftObjectPtr` "/Game/Levels/Experiment_2.Experiment_2"))))
    (:`Hello`
      (`self.FadeToBlack`)
      (`self.Invisible Scene`)
      (`GameplayStatics.OpenLevelBySoftObjectPtr` "/Game/Levels/Home.Home"))))

(fn `FadeIntoScene`
  (bind _returnvalue (`GameplayStatics.GetActorOfClass` "/Script/LevelSequence.LevelSequenceActor"))
  (`LevelSequenceActor.SetSequence` _returnvalue "/Game/Sequences/FadeIn.FadeIn")
  (`MovieSceneSequencePlayer.Play` (`LevelSequenceActor.SequencePlayer` _returnvalue)))

(fn `FadeToBlack`
  (bind _returnvalue (`GameplayStatics.GetActorOfClass` "/Script/LevelSequence.LevelSequenceActor"))
  (`LevelSequenceActor.SetSequence` _returnvalue "/Game/Sequences/FadeOut.FadeOut")
  (`MovieSceneSequencePlayer.Play` (`LevelSequenceActor.SequencePlayer` _returnvalue)))

(fn `Get Object Looking At As ScreenButton`
  (returns (`ScreenButton Object` :type "/Game/Blueprints/ScreenButton Object Reference"))
  (bind _asbp_fps_character (cast `/Game/Blueprints/BP_FPS_Character` (`GameplayStatics.GetPlayerCharacter` 0)))
  (bind _asscreen_button (cast `/Game/Blueprints/ScreenButton` (`/Game/Blueprints/BP_FPS_Character.ObjectLookingAt` _asbp_fps_character)))
  (return _asscreen_button))

(fn `Invisible Scene`
  (bind _returnvalue (`GameplayStatics.GetActorOfClass` "/Script/LevelSequence.LevelSequenceActor"))
  (`LevelSequenceActor.SetSequence` _returnvalue "/Game/Sequences/InvisibleScreen.InvisibleScreen")
  (`MovieSceneSequencePlayer.Play` (`LevelSequenceActor.SequencePlayer` _returnvalue)))

(fn `UserConstructionScript`)

(fn `Visible Scene`
  (bind _returnvalue (`GameplayStatics.GetActorOfClass` "/Script/LevelSequence.LevelSequenceActor"))
  (`LevelSequenceActor.SetSequence` _returnvalue "/Game/Sequences/VisibleScreen.VisibleScreen")
  (`MovieSceneSequencePlayer.Play` (`LevelSequenceActor.SequencePlayer` _returnvalue)))