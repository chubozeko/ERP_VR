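; ExemplarObject is a data-holder Blueprint describing one exemplar by name, type, material and a flag for whether it is a good exemplar.
; CreateExemplarObject acts as an initializer that stores all four values in member variables.
; Getter functions expose the name, material and good-exemplar flag, while the type has no getter here.
; The event graph and construction script contain no logic.
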(fn `Create Exemplar Object`
  (params (Name :type String) (Type :type "/Game/Scripts/ExemplarTypes Enum" :default "NewEnumerator0") (Material :type "Material Object Reference") (isAGoodExempler :type Boolean))
  (set `self.Exemplar Name` Name)
  (set `self.Exemplar Type` Type)
  (set `self.Material` Material)
  (set `self.isGoodExemplar` isAGoodExempler))

(fn `Get Exemplar Name`
  (returns (`Exemplar Name` :type String))
  (return (`self.Exemplar Name`)))

(fn `Get Material`
  (returns (Material :type "Material Object Reference"))
  (return (`self.Material`)))

(fn `Is A Good Exemplar`
  (returns (IsGoodExemplar :type Boolean))
  (return (`self.isGoodExemplar`)))

(fn `UserConstructionScript`)