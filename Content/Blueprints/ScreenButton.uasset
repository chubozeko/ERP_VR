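; VR world-space button that hands its press to an ERP, trial or rating controller.
; Box overlap by a VRUser with exactly one hand grabbing registers it as the looked-at object and triggers hover feedback through border material or text size.
; InteractwithObject selects it and calls the controller.
; In press-and-hold mode, Tick grows the border while held, then marks it selected and shows loading text without calling the controller.
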(event `self.ReceiveBeginPlay`
  (bind _buttonborder (`self.ButtonBorder`))
  (bind (_relativescale3d_x _relativescale3d_y) (`KismetMathLibrary.BreakVector` (`SceneComponent.RelativeScale3D` (`self.ButtonBorder`))))
  (bind _returnvalue (`MaterialInterface.GetBaseMaterial` (`PrimitiveComponent.GetMaterial` (`self.Button`) 0)))
  (set `self.Button Base Material` _returnvalue)
  (bind _returnvalue_2 (`MaterialInterface.GetBaseMaterial` (`PrimitiveComponent.GetMaterial` (`self.ButtonBorder`) 0)))
  (set `self.Button Material` _returnvalue_2)
  (if (`self.Press and Hold Button`)
    (bind _output_get (set `self.Hold Y Scale` _relativescale3d_y))
    (`SceneComponent.SetWorldScale3D` _buttonborder (`KismetMathLibrary.MakeVector` (.x (`SceneComponent.K2_GetComponentScale` _buttonborder)) _output_get (.z (`SceneComponent.K2_GetComponentScale` _buttonborder))))
    (set `self.Original Font Size` (.z (`TextRenderComponent.GetTextWorldSize` (`self.ButtonText`))))
    (else
      (`PrimitiveComponent.SetMaterial` _buttonborder 0 (`self.Button Base Material`)))))

(event `self.InteractWithObject`
  (set `self.IsSelected` true)
  (`self.Execute Button Function`))

(event `self.Box.OnComponentBeginOverlap`
  (params (OverlappedComponent :type "PrimitiveComponent Object Reference") (OtherActor :type "Actor Object Reference") (OtherComp :type "PrimitiveComponent Object Reference") (OtherBodyIndex :type Integer) (bFromSweep :type Boolean) (SweepResult :type "HitResult Structure (by ref)"))
  (if (not (`self.bHidden`))
    (bind _asvruser (cast `/Game/Blueprints/Players/VRUser` OtherActor))
    (if (xor (`/Game/Blueprints/Players/VRUser.Is Grabbing Left` _asvruser) (`/Game/Blueprints/Players/VRUser.Is Grabbing Right` _asvruser))
      (set `/Game/Blueprints/Players/VRUser.Object Looking At` self _asvruser)
      (`self.On Button Hover Enter`))))

(event `self.Box.OnComponentEndOverlap`
  (params (OverlappedComponent :type "PrimitiveComponent Object Reference") (OtherActor :type "Actor Object Reference") (OtherComp :type "PrimitiveComponent Object Reference") (OtherBodyIndex :type Integer))
  (bind _asvruser (cast `/Game/Blueprints/Players/VRUser` OtherActor))
  (set `/Game/Blueprints/Players/VRUser.Object Looking At` null _asvruser)
  (`self.On Button Hover Exit`))

(event `self.ReceiveTick`
  (params (DeltaSeconds :type "Float (single-precision)"))
  (bind _buttonborder (`self.ButtonBorder`))
  (bind _returnvalue (`SceneComponent.K2_GetComponentScale` _buttonborder))
  (bind _returnvalue_2 (+ (`self.Hold Y Scale`) 0.01))
  (bind _returnvalue_3 (< _returnvalue_2 (`self.Hold End Y Scale`)))
  (if (and (`self.Press and Hold Button`) (`self.Is Hover Entered`))
    (if (`self.Is Button Held`)
      (if _returnvalue_3
        (bind _output_get (set `self.Hold Y Scale` _returnvalue_2))
        (`SceneComponent.SetWorldScale3D` _buttonborder (`KismetMathLibrary.MakeVector` (.x _returnvalue) _output_get (.z _returnvalue)))
        (else
          (set `self.IsSelected` true)
          (`TextRenderComponent.K2_SetText` (`self.ButtonText`) (`KismetTextLibrary.Conv_StringToText` "Loading..."))))
      (elif _returnvalue_3
        (bind _output_get_2 (set `self.Hold Y Scale` (`self.Hold Start Y Scale`)))
        (`SceneComponent.SetWorldScale3D` _buttonborder (`KismetMathLibrary.MakeVector` (.x _returnvalue) _output_get_2 (.z _returnvalue)))))))

(fn `Execute Button Function`
  (bind _controller (`self.Controller`))
  (bind _aserp_controller (cast `/Game/Blueprints/LevelControllers/ERP_Controller` _controller)
    (:`then`
      (`/Game/Blueprints/LevelControllers/ERP_Controller.Execute Button Function` _aserp_controller self))
    (:`CastFailed`
      (bind _asetrial_controller (cast `/Game/Blueprints/LevelControllers/ETrialController` _controller)
        (:`then`
          (`/Game/Blueprints/LevelControllers/ETrialController.Execute Button Function` _asetrial_controller self))
        (:`CastFailed`
          (bind _aserating_controller (cast `/Game/Blueprints/LevelControllers/ERatingController` _controller))
          (`/Game/Blueprints/LevelControllers/ERatingController.Execute Button Function` _aserating_controller self))))))

(fn `On Button Hover Enter`
  (set `self.Is Hover Entered` true)
  (if (`self.Press and Hold Button`)
    (`TextRenderComponent.SetWorldSize` (`self.ButtonText`) (* (`self.Original Font Size`) 1.15))
    (else
      (`PrimitiveComponent.SetMaterial` (`self.ButtonBorder`) 0 (`self.Button Material`)))))

(fn `On Button Hover Exit`
  (set `self.Is Hover Entered` false)
  (if (`self.Press and Hold Button`)
    (`TextRenderComponent.SetWorldSize` (`self.ButtonText`) (* (`self.Original Font Size`) 0.85))
    (else
      (`PrimitiveComponent.SetMaterial` (`self.ButtonBorder`) 0 (`self.Button Base Material`)))))

(fn `UserConstructionScript`)