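; Level controller that runs one VR experiment trial, showing a crosshair and exemplar room, preceded by a cue word in the second experiment type.
; On BeginPlay it loads the VRUser's save and applies the current trial's exemplar and cue word.
; Delay-chained phases use Level Sequence fades, teleport the user, timestamp exemplar viewing, save, then open Experiment_Trial.
; Millisecond intervals from the GameInstance are integer-divided, truncating to whole seconds.
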(event `self.ReceiveBeginPlay`
  ;[0.2346 0.08438 0.2961 0.502 14] Load Session from Character
  (`self.Invisible Scene`)
  (`KismetSystemLibrary.Delay` 0.2)
  (bind _asvruser (cast `/Game/Blueprints/Players/VRUser` (`GameplayStatics.GetPlayerPawn` 0)))
  (bind _output_get (set `self.As VRUser` _asvruser))
  (`/Game/Blueprints/Players/VRUser.Load Session` _output_get self (`/Game/Blueprints/Players/GI_Experiments.Save Slot Name` (`/Game/Blueprints/Players/VRUser.GameInstance` _asvruser)))
  ;[0.2346 0.08438 0.2961 0.502 14] Set Exemplar Room material
  (bind _assave_experiments (cast `/Game/Blueprints/Players/Save_Experiments` (`/Game/Blueprints/Players/VRUser.Save REF` (`self.As VRUser`))))
  (bind _trial_index (`/Game/Blueprints/Players/Save_Experiments.Get Current Trial Index` _assave_experiments))
  (bind _output_get_2 (set `self.Current Trial Index` _trial_index))
  (bind _exemplar_name (`/Game/Blueprints/Players/Save_Experiments.Get Exemplar Name with Index` _assave_experiments _output_get_2))
  (bind _outactors (`GameplayStatics.GetAllActorsOfClass` "/Game/Blueprints/ExemplarObject.ExemplarObject_C"))
  (for _array_element _outactors
    (bind _exemplar_name_2 (`/Game/Blueprints/ExemplarObject.Get Exemplar Name` _array_element))
    (if (== _exemplar_name_2 _exemplar_name)
      (`/Game/Blueprints/ExemplarRoom.Set Viewing Globe Material` (`self.ExemplarRoom`) _array_element)
      (break)))
  ;[0.2346 0.08438 0.2961 0.502 14] Set Cue Word
  (bind _cue_word (`/Game/Blueprints/Players/Save_Experiments.Get Cue Word with Index` _assave_experiments _output_get_2))
  (set `self.Current Trial Cue Word` _cue_word)
  ;[0.2346 0.08438 0.2961 0.502 14] Run Experiment
  (if (`|EnumEquality` (`self.Experiment Type`) "NewEnumerator0")
    (`self.Event Run Experiment 1`)
    (else
      (`self.Event Run Experiment 2`))))

(event `Event Run Experiment 1`
  (bind _as_vruser (`self.As VRUser`))
  (bind _gameinstance (`/Game/Blueprints/Players/VRUser.GameInstance` (`self.As VRUser`)))
  (bind _interval_in_seconds (`self.Convert Interval to Seconds` (`/Game/Blueprints/Players/GI_Experiments.Fade Interval` _gameinstance))) ; Fade Interval
  (bind _interval_in_seconds_2 (`self.Convert Interval to Seconds` (`/Game/Blueprints/Players/GI_Experiments.Crosshair Interval` _gameinstance))) ; Crosshair Interval
  (bind _interval_in_seconds_3 (`self.Convert Interval to Seconds` (`/Game/Blueprints/Players/GI_Experiments.Exemplar Interval` _gameinstance))) ; Exemplar
  ;[0.4 1 0.3569 0.5 14] Fade In -> Show Crosshair -> Fade Out
  (`self.View Crosshair`)
  (`KismetSystemLibrary.Delay` _interval_in_seconds)
  (`self.FadeIntoScene`)
  (`KismetSystemLibrary.Delay` _interval_in_seconds_2)
  (`self.FadeToBlack`)
  ;[0.4039 1 0.3569 0.502 14] Move to Exemplar Room -> Show Exemplar -> Fade Out
  (`KismetSystemLibrary.Delay` _interval_in_seconds)
  (`self.Teleport to Exemplar Room`)
  (`KismetSystemLibrary.Delay` _interval_in_seconds)
  (`self.FadeIntoScene`)
  (set `self.Exemplar Start Time` (`KismetMathLibrary.Now`))
  (`KismetSystemLibrary.Delay` _interval_in_seconds_3)
  (`self.FadeToBlack`)
  (set `self.Exemplar End Time` (`KismetMathLibrary.Now`))
  (`KismetSystemLibrary.Delay` _interval_in_seconds)
  (`/Game/Blueprints/Players/VRUser.Save Session` _as_vruser (`/Game/Blueprints/Players/GI_Experiments.Save Slot Name` (`/Game/Blueprints/Players/VRUser.GameInstance` _as_vruser)))
  (`GameplayStatics.OpenLevelBySoftObjectPtr` "/Game/Levels/Experiment_Trial.Experiment_Trial"))

(event `Event Run Experiment 2`
  (bind _as_vruser (`self.As VRUser`))
  (bind _gameinstance (`/Game/Blueprints/Players/VRUser.GameInstance` (`self.As VRUser`)))
  (bind _interval_in_seconds (`self.Convert Interval to Seconds` (`/Game/Blueprints/Players/GI_Experiments.Fade Interval` _gameinstance))) ; Fade Interval
  (bind _interval_in_seconds_2 (`self.Convert Interval to Seconds` (`/Game/Blueprints/Players/GI_Experiments.Crosshair Interval` _gameinstance))) ; Crosshair Interval
  (bind _interval_in_seconds_3 (`self.Convert Interval to Seconds` (`/Game/Blueprints/Players/GI_Experiments.Exemplar Interval` _gameinstance))) ; Exemplar Interval
  (bind _interval_in_seconds_4 (`self.Convert Interval to Seconds` (`/Game/Blueprints/Players/GI_Experiments.Cue Word Interval` _gameinstance))) ; Cue Word Interval
  ;[0.2824 1 0.9804 0.502 14] Fade In -> View Cue Word -> Fade Out
  (`self.View Cue Word`)
  (`KismetSystemLibrary.Delay` _interval_in_seconds)
  (`self.FadeIntoScene`)
  (`KismetSystemLibrary.Delay` _interval_in_seconds_4)
  (`self.FadeToBlack`)
  (`KismetSystemLibrary.Delay` _interval_in_seconds)
  ;[0.2824 1 0.9804 0.502 14] Fade In -> View Crosshair -> Fade Out
  (`self.View Crosshair`)
  (`KismetSystemLibrary.Delay` _interval_in_seconds)
  (`self.FadeIntoScene`)
  (`KismetSystemLibrary.Delay` _interval_in_seconds_2)
  (`self.FadeToBlack`)
  (`KismetSystemLibrary.Delay` _interval_in_seconds)
  ;[0.2824 1 0.9804 0.502 14] Move to Exemplar Room -> Fade In -> Show Exemplar Room -> Fade Out
  (`self.Teleport to Exemplar Room`)
  (`KismetSystemLibrary.Delay` _interval_in_seconds)
  (`self.FadeIntoScene`)
  (set `self.Exemplar Start Time` (`KismetMathLibrary.Now`))
  (`KismetSystemLibrary.Delay` _interval_in_seconds_3)
  (`self.FadeToBlack`)
  (set `self.Exemplar End Time` (`KismetMathLibrary.Now`))
  (`KismetSystemLibrary.Delay` _interval_in_seconds)
  (`/Game/Blueprints/Players/VRUser.Save Session` _as_vruser (`/Game/Blueprints/Players/GI_Experiments.Save Slot Name` (`/Game/Blueprints/Players/VRUser.GameInstance` _as_vruser)))
  (`GameplayStatics.OpenLevelBySoftObjectPtr` "/Game/Levels/Experiment_Trial.Experiment_Trial"))

(fn `Convert Interval to Seconds`
  (params (`Interval in Milliseconds` :type "Float (double-precision)"))
  (returns (`Interval in Seconds` :type "Float (double-precision)"))
  (return (`KismetMathLibrary.Conv_IntToDouble` (/ `Interval in Milliseconds` 1000))))

(fn `FadeIntoScene`
  (bind _returnvalue (`GameplayStatics.GetActorOfClass` "/Script/LevelSequence.LevelSequenceActor"))
  (`LevelSequenceActor.SetSequence` _returnvalue "/Game/Sequences/FadeIn.FadeIn")
  (`MovieSceneSequencePlayer.Play` (`LevelSequenceActor.SequencePlayer` _returnvalue)))

(fn `FadeToBlack`
  (bind _returnvalue (`GameplayStatics.GetActorOfClass` "/Script/LevelSequence.LevelSequenceActor"))
  (`LevelSequenceActor.SetSequence` _returnvalue "/Game/Sequences/FadeOut.FadeOut")
  (`MovieSceneSequencePlayer.Play` (`LevelSequenceActor.SequencePlayer` _returnvalue)))

(fn `Invisible Scene`
  (bind _returnvalue (`GameplayStatics.GetActorOfClass` "/Script/LevelSequence.LevelSequenceActor"))
  (`LevelSequenceActor.SetSequence` _returnvalue "/Game/Sequences/InvisibleScreen.InvisibleScreen")
  (`MovieSceneSequencePlayer.Play` (`LevelSequenceActor.SequencePlayer` _returnvalue)))

(fn `Teleport to Exemplar Room`
  (bind _asvruser (cast `/Game/Blueprints/Players/VRUser` (`GameplayStatics.GetPlayerPawn` 0)))
  (`self.K2_SetActorLocation` _asvruser (`KismetMathLibrary.TransformLocation` (`self.Exemplar Room Position`)) false true))

(fn `UserConstructionScript`)

(fn `View Crosshair`
  (bind _crosshair (`self.Crosshair`))
  (bind _question (`self.Question`))
  (`TextRenderComponent.K2_SetText` (`TextRenderActor.TextRender` _crosshair) (`KismetTextLibrary.Conv_StringToText` "+"))
  (`self.SetActorHiddenInGame` _crosshair false)
  (if (`KismetSystemLibrary.IsValid` _question)
    (`self.SetActorHiddenInGame` _question true)))

(fn `View Cue Word`
  (bind _question (`self.Question`))
  (`TextRenderComponent.K2_SetText` (`TextRenderActor.TextRender` _question) (`KismetTextLibrary.Conv_StringToText` (`self.Current Trial Cue Word`)))
  (`self.SetActorHiddenInGame` _question false)
  (`self.SetActorHiddenInGame` (`self.Crosshair`) true))

(fn `Visible Scene`
  (bind _returnvalue (`GameplayStatics.GetActorOfClass` "/Script/LevelSequence.LevelSequenceActor"))
  (`LevelSequenceActor.SetSequence` _returnvalue "/Game/Sequences/VisibleScreen.VisibleScreen")
  (`MovieSceneSequencePlayer.Play` (`LevelSequenceActor.SequencePlayer` _returnvalue)))