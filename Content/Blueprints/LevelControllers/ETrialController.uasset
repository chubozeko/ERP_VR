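; Level controller for the VR experiment's response screen, asking a two-choice question about a depiction or cue-word match, depending on experiment ID.
; BeginPlay loads the session from VRUser (or a debug FPS character), sets question text, then fades in by swapping Level Sequences.
; ExecuteButtonFunction records answer and timing, saves, and shows completion.
; Continue reopens the experiment level; when no trials remain, results are exported and the screen fades out.
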(event `self.ReceiveBeginPlay`
  (`self.Invisible Scene`)
  (`KismetSystemLibrary.Delay` 0.2)
  (bind _asvruser (cast `/Game/Blueprints/Players/VRUser` (`GameplayStatics.GetPlayerPawn` 0))
    (:`then`
      (bind _output_get (set `self.As VRUser` _asvruser))
      (bind _gameinstance (`/Game/Blueprints/Players/VRUser.GameInstance` _output_get))
      (`/Game/Blueprints/Players/VRUser.Load Session` _output_get self (`/Game/Blueprints/Players/GI_Experiments.Save Slot Name` _gameinstance)))
    (:`CastFailed`
      ;[0.06663 0.05448 0.2918 0.749 14] FPS Controller (for debugging)
      (bind _asbp_fps_character (cast `/Game/Blueprints/Players/BP_FPS_Character` (`GameplayStatics.GetPlayerCharacter` 0)))
      (bind _output_get_2 (set `self.As BP FPS Character` _asbp_fps_character))
      (`/Game/Blueprints/Players/BP_FPS_Character.Load Session` _output_get_2 self (`/Game/Blueprints/Players/GI_Experiments.Save Slot Name` (`/Game/Blueprints/Players/BP_FPS_Character.GameInstance` _output_get_2)))))
  (switch `int` (`self.Experiment ID`)
    (:`1`
      (`self.View Experiment 1 Question`))
    (:`2`
      (`self.View Experiment 2 Question`)))
  (`self.K2_SetActorLocation` (`self.Menu Panel`) (0.0 1085.0 150.0) false true)
  (bind _interval_in_seconds (`self.Convert Interval to Seconds` (`/Game/Blueprints/Players/GI_Experiments.Fade Interval` _gameinstance))) ; Fade Interval
  (`KismetSystemLibrary.Delay` _interval_in_seconds)
  (`self.FadeIntoScene`)
  (set `self.Response Start Time` (`KismetMathLibrary.Now`))
  (`/Game/Blueprints/Players/VRUser.Set Motion Controller Visibility` (`self.As VRUser`) true))

(event `View Experiment 1 Question`
  (bind _question (`self.Question`))
  (bind _answer_l (`self.Answer L`))
  (bind _answer_r (`self.Answer R`))
  (bind _exemplar_type (`self.Exemplar Type`))
  (bind _crosshair (`self.Crosshair`))
  ;[0.06663 0.05448 0.2918 0.749 14] View Experiment 1 Question
  (`TextRenderComponent.K2_SetText` (`TextRenderActor.TextRender` _crosshair) (`KismetTextLibrary.Conv_StringToText` "+"))
  (`self.SetActorHiddenInGame` _crosshair false)
  (`TextRenderComponent.K2_SetText` (`TextRenderActor.TextRender` _answer_l) (`KismetTextLibrary.Conv_StringToText` "GOOD"))
  (`self.SetActorHiddenInGame` _answer_l false)
  (`TextRenderComponent.K2_SetText` (`TextRenderActor.TextRender` _answer_r) (`KismetTextLibrary.Conv_StringToText` "BAD"))
  (`self.SetActorHiddenInGame` _answer_r false)
  (bind _correct_article (`self.Get Article for Word` _exemplar_type))
  (`TextRenderComponent.K2_SetText` (`TextRenderActor.TextRender` _question) (`KismetTextLibrary.Conv_StringToText` (`KismetStringLibrary.Concat_StrStr` "Was that a GOOD or BAD depiction of " _correct_article " <br> " _exemplar_type "?")))
  (`self.SetActorHiddenInGame` _question false))

(event `View Experiment 2 Question`
  (bind _question (`self.Question`))
  (bind _crosshair (`self.Crosshair`))
  (bind _answer_l (`self.Answer L`))
  (bind _answer_r (`self.Answer R`))
  ;[0.06667 0.0549 0.2902 0.749 14] View Experiment 2 Question
  (`TextRenderComponent.K2_SetText` (`TextRenderActor.TextRender` _crosshair) (`KismetTextLibrary.Conv_StringToText` "+"))
  (`self.SetActorHiddenInGame` _crosshair false)
  (`TextRenderComponent.K2_SetText` (`TextRenderActor.TextRender` _answer_l) (`KismetTextLibrary.Conv_StringToText` "YES"))
  (`self.SetActorHiddenInGame` _answer_l false)
  (`TextRenderComponent.K2_SetText` (`TextRenderActor.TextRender` _answer_r) (`KismetTextLibrary.Conv_StringToText` "NO"))
  (`self.SetActorHiddenInGame` _answer_r false)
  (`TextRenderComponent.K2_SetText` (`TextRenderActor.TextRender` _question) (`KismetTextLibrary.Conv_StringToText` (`KismetStringLibrary.Concat_StrStr` "Do you think the Cue Word \"" (`self.Cue Word`) "\" matched the given scene?")))
  (`self.SetActorHiddenInGame` _question false))

(event `View Experiment Complete`
  (bind _menu_panel (`self.Menu Panel`))
  (bind _continue (`self.Continue`))
  ;[0.06663 0.05448 0.2918 0.749 14] View Experiment Trial Complete
  (`self.SetActorHiddenInGame` (`self.Crosshair`) true)
  (`self.SetActorHiddenInGame` (`self.Answer L`) true)
  (`self.SetActorHiddenInGame` (`self.Answer R`) true)
  (`self.SetActorHiddenInGame` (`self.Question`) true)
  (`self.SetActorHiddenInGame` (`self.Trial Complete`) false)
  (for _array_element (`self.Response Buttons`)
    (`self.SetActorHiddenInGame` _array_element true))
  (switch `int` (`/Game/Blueprints/Players/GI_Experiments.Trial Number to Run` (`/Game/Blueprints/Players/VRUser.GameInstance` (`self.As VRUser`)))
    (:`Default`
      (`self.SetActorHiddenInGame` _continue false)
      (`self.K2_SetActorLocation` _menu_panel (-400.0 1085.0 150.0) false true))
    (:`0`
      (`self.SetActorHiddenInGame` _continue true)
      (`self.K2_SetActorLocation` _menu_panel (400.0 1085.0 150.0) false true)
      (`/Game/Blueprints/Players/VRUser.Save and Export Trials` (`self.As VRUser`))
      (`KismetSystemLibrary.Delay` 5.0)
      (`self.FadeToBlack`)
      (`self.Invisible Scene`))))

(fn `Convert Interval to Seconds`
  (params (`Interval in Milliseconds` :type "Float (double-precision)"))
  (returns (`Interval in Seconds` :type "Float (double-precision)"))
  (return (`KismetMathLibrary.Conv_IntToDouble` (/ `Interval in Milliseconds` 1000))))

(fn `Execute Button Function`
  (params (Button :type "/Game/Blueprints/ScreenButton Object Reference"))
  (bind _as_vruser (`self.As VRUser`))
  (bind _experiment_id (`self.Experiment ID`))
  (switch `string` (`/Game/Blueprints/ScreenButton.Button Function` Button)
    (:`AnswerPositive`
      (switch `int` _experiment_id
        (:`1`
          (set `self.Response` "GOOD"))
        (:`2`
          (set `self.Response` "YES")))
      (set `self.Response End Time` (`KismetMathLibrary.Now`) :!label _label)
      (`/Game/Blueprints/Players/VRUser.Save Session` _as_vruser (`/Game/Blueprints/Players/GI_Experiments.Save Slot Name` (`/Game/Blueprints/Players/VRUser.GameInstance` _as_vruser)))
      (`self.View Experiment Complete`))
    (:`AnswerNegative`
      (switch `int` _experiment_id
        (:`1`
          (set `self.Response` "BAD")
          (goto _label))
        (:`2`
          (set `self.Response` "NO")
          (goto _label))))
    (:`ContinueToNextTrial`
      (`self.FadeToBlack`)
      (`self.Invisible Scene`)
      (switch `int` (`self.Experiment ID`)
        (:`1`
          (`GameplayStatics.OpenLevelBySoftObjectPtr` "/Game/Levels/Experiment_1.Experiment_1"))
        (:`2`
          (`GameplayStatics.OpenLevelBySoftObjectPtr` "/Game/Levels/Experiment_2.Experiment_2"))))))

(fn `FadeIntoScene`
  (bind _returnvalue (`GameplayStatics.GetActorOfClass` "/Script/LevelSequence.LevelSequenceActor"))
  (`LevelSequenceActor.SetSequence` _returnvalue "/Game/Sequences/FadeIn.FadeIn")
  (`MovieSceneSequencePlayer.Play` (`LevelSequenceActor.SequencePlayer` _returnvalue)))

(fn `FadeToBlack`
  (bind _returnvalue (`GameplayStatics.GetActorOfClass` "/Script/LevelSequence.LevelSequenceActor"))
  (`LevelSequenceActor.SetSequence` _returnvalue "/Game/Sequences/FadeOut.FadeOut")
  (`MovieSceneSequencePlayer.Play` (`LevelSequenceActor.SequencePlayer` _returnvalue)))

(fn `Get Article for Word`
  (params (Word :type String))
  (returns (`Correct Article` :type String))
  (locals (`Article to Use` :type String))
  (if (`KismetStringLibrary.Contains` "AEIOU" (`|GetArrayItem` (`KismetStringLibrary.GetCharacterArrayFromString` Word)))
    (set `local.Article to Use` "an")
    (else
      (set `local.Article to Use` "a")))
  (return (`local.Article to Use`)))

(fn `Get Object Looking At As ScreenButton`
  (returns (`ScreenButton Object` :type "/Game/Blueprints/ScreenButton Object Reference"))
  (bind _asvruser (cast `/Game/Blueprints/Players/VRUser` (`GameplayStatics.GetPlayerPawn` 0)))
  (bind _asscreen_button (cast `/Game/Blueprints/ScreenButton` (`/Game/Blueprints/Players/VRUser.Object Looking At` _asvruser)))
  (return _asscreen_button))

(fn `Invisible Scene`
  (bind _returnvalue (`GameplayStatics.GetActorOfClass` "/Script/LevelSequence.LevelSequenceActor"))
  (`LevelSequenceActor.SetSequence` _returnvalue "/Game/Sequences/InvisibleScreen.InvisibleScreen")
  (`MovieSceneSequencePlayer.Play` (`LevelSequenceActor.SequencePlayer` _returnvalue)))

(fn `UserConstructionScript`)

(fn `Visible Scene`
  (bind _returnvalue (`GameplayStatics.GetActorOfClass` "/Script/LevelSequence.LevelSequenceActor"))
  (`LevelSequenceActor.SetSequence` _returnvalue "/Game/Sequences/VisibleScreen.VisibleScreen")
  (`MovieSceneSequencePlayer.Play` (`LevelSequenceActor.SequencePlayer` _returnvalue)))