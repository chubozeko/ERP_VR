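; Level controller for a VR experiment menu that launches Experiment 1 or 2, or quits, from selected gaze-targeted screen buttons.
; Tick polls the VRUser's looked-at button; choosing an experiment spawns trials from shuffled exemplars, saves a newly named session and opens that level.
; Experiment 2 uses only good exemplars, assigning random cue words steered toward a matched/unmatched percentage.
; Helpers teleport the user between rooms and play Level Sequence screen fades.
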(event `self.ReceiveBeginPlay`
  (`self.Invisible Scene`)
  (`KismetSystemLibrary.Delay` 1.0)
  (`self.FadeIntoScene`))

(event `self.ReceiveTick`
  (params (DeltaSeconds :type "Float (single-precision)"))
  ;[0 0.3763 0.02029 0.502 14] Check for Object being Looked at
  (for _array_element (`self.Experiments Buttons`)
    (bind _screenbutton_object (`self.Get Object Looking At As ScreenButton`))
    (if (and (== _screenbutton_object _array_element) (`/Game/Blueprints/ScreenButton.IsSelected` _array_element))
      (`self.Execute Button Function` _array_element)
      (set `/Game/Blueprints/ScreenButton.IsSelected` false _array_element))))

(fn `Convert Interval to Seconds`
  (params (`Interval in Milliseconds` :type "Float (double-precision)"))
  (returns (`Interval in Seconds` :type "Float (double-precision)"))
  (return (`KismetMathLibrary.Conv_IntToDouble` (/ `Interval in Milliseconds` 1000))))

(fn `Deselect All Buttons`
  (for _array_element (`self.Experiments Buttons`)
    (set `/Game/Blueprints/ScreenButton.IsSelected` false _array_element)))

(fn `Execute Button Function`
  (params (Button :type "/Game/Blueprints/ScreenButton Object Reference"))
  (switch `string` (`/Game/Blueprints/ScreenButton.Button Function` Button)
    (:`Exp1`
      (`self.Initialize Experiment 1 Trials`)
      (`self.Set Up Experiment` "NewEnumerator0")
      (`self.Deselect All Buttons`)
      (`GameplayStatics.OpenLevelBySoftObjectPtr` "/Game/Levels/Experiment_1.Experiment_1"))
    (:`Exp2`
      (`self.Initialize Experiment 2 Trials`)
      (`self.Set Up Experiment` "NewEnumerator1")
      (`self.Deselect All Buttons`)
      (`GameplayStatics.OpenLevelBySoftObjectPtr` "/Game/Levels/Experiment_2.Experiment_2"))
    (:`Quit`
      (`KismetSystemLibrary.QuitGame` null "Quit"))))

(fn `FadeIntoScene`
  (bind _returnvalue (`GameplayStatics.GetActorOfClass` "/Script/LevelSequence.LevelSequenceActor"))
  (`LevelSequenceActor.SetSequence` _returnvalue "/Game/Sequences/FadeIn.FadeIn")
  (`MovieSceneSequencePlayer.Play` (`LevelSequenceActor.SequencePlayer` _returnvalue)))

(fn `FadeToBlack`
  (bind _returnvalue (`GameplayStatics.GetActorOfClass` "/Script/LevelSequence.LevelSequenceActor"))
  (`LevelSequenceActor.SetSequence` _returnvalue "/Game/Sequences/FadeOut.FadeOut")
  (`MovieSceneSequencePlayer.Play` (`LevelSequenceActor.SequencePlayer` _returnvalue)))

(fn `Get Object Looking At As ScreenButton`
  (returns (`ScreenButton Object` :type "/Game/Blueprints/ScreenButton Object Reference"))
  (bind _asvruser (cast `/Game/Blueprints/Players/VRUser` (`GameplayStatics.GetPlayerPawn` 0)))
  (bind _asscreen_button (cast `/Game/Blueprints/ScreenButton` (`/Game/Blueprints/Players/VRUser.Object Looking At` _asvruser)))
  (return _asscreen_button))

(fn `Initialize Experiment 1 Trials`
  (bind _exemplars (`self.Exemplars`))
  (`KismetArrayLibrary.Array_Shuffle` _exemplars)
  (for (_array_element _array_index) _exemplars
    (bind _returnvalue (`|SpawnActorFromClass` "/Game/Blueprints/ExperimentTrial.ExperimentTrial_C" (`self.GetTransform` self) "Undefined" "OverrideRootScale" null null))
    (bind _trial (`/Game/Blueprints/ExperimentTrial.Initialize Trial` _returnvalue _array_index _array_element "NewEnumerator0" ""))
    (`KismetArrayLibrary.Array_Add` (`self.Experiment 1 Trials`) _trial)))

(fn `Initialize Experiment 2 Trials`
  (locals (`New Trial` :type "/Game/Blueprints/ExperimentTrial Object Reference") (`New Cue Word` :type String) (`Total Matched CW` :type Integer) (`Matched CW Count` :type Integer :default 0) (`Total Unmatched CW` :type Integer) (`Unmatched CW Count` :type Integer :default 0))
  (bind _exemplars (`self.Exemplars`))
  (bind _returnvalue (`KismetArrayLibrary.Array_Length` _exemplars))
  (`KismetArrayLibrary.Array_Shuffle` _exemplars)
  (`KismetArrayLibrary.Array_Clear` (`self.Experiment 2 Trials`))
  (bind _output_get (set `local.Total Matched CW` (`KismetMathLibrary.FFloor` (* (`KismetMathLibrary.Conv_IntToDouble` _returnvalue) (/ (`self.Matched Percentage`) 100.0)))))
  (set `local.Total Unmatched CW` (- _returnvalue _output_get))
  (for (_array_element _array_index) _exemplars
    (bind _isgoodexemplar (`/Game/Blueprints/ExemplarObject.Is A Good Exemplar` _array_element))
    (if _isgoodexemplar
      (bind _returnvalue_2 (`|SpawnActorFromClass` "/Game/Blueprints/ExperimentTrial.ExperimentTrial_C" (`self.GetTransform` self) "Undefined" "OverrideRootScale" null null))
      (bind _cue_word (`self.Select Cue Word from Exemplar Types`))
      (set `local.New Cue Word` _cue_word)
      (bind _returnvalue_3 (`|GetEnumeratorNameAsString` (`/Game/Blueprints/ExemplarObject.Exemplar Type` _array_element)))
      (bind _returnvalue_4 (`KismetStringLibrary.EqualEqual_StrStr` (`local.New Cue Word`) _returnvalue_3))
      (if _returnvalue_4
        (if (< (`local.Matched CW Count`) (`local.Total Matched CW`))
          (bind _result (`/Engine/EditorBlueprintResources/StandardMacros.IncrementInt` (`local.Matched CW Count`))
            (:`  `
              (set `local.Matched CW Count` _result)))
          (else
            (while (not _returnvalue_4)
              (bind _cue_word_2 (`self.Select Cue Word from Exemplar Types`))
              (set `local.New Cue Word` _cue_word_2))))
        (elif (< (`local.Unmatched CW Count`) (`local.Total Unmatched CW`))
          (bind _result_2 (`/Engine/EditorBlueprintResources/StandardMacros.IncrementInt` (`local.Unmatched CW Count`))
            (:`  `
              (set `local.Unmatched CW Count` _result_2)))
          (else
            (set `local.New Cue Word` _returnvalue_3)
            (bind _result_3 (`/Engine/EditorBlueprintResources/StandardMacros.IncrementInt` (`local.Matched CW Count`))
              (:`  `
                (set `local.Matched CW Count` _result_3))))))
      (bind _trial (`/Game/Blueprints/ExperimentTrial.Initialize Trial` _returnvalue_2 _array_index _array_element "NewEnumerator1" (`local.New Cue Word`)))
      (bind _output_get_2 (set `local.New Trial` _trial))
      (`KismetArrayLibrary.Array_Add` (`self.Experiment 2 Trials`) _output_get_2)))
  (`KismetSystemLibrary.PrintString` (`KismetStringLibrary.Concat_StrStr` "[EXP 2] " (`KismetStringLibrary.Conv_IntToString` (`KismetArrayLibrary.Array_Length` (`self.Experiment 2 Trials`))) " Experiment Trials CREATED!") false true (struct :`G` 0.66 :`B` 1.0 :`A` 1.0) 5.0))

(fn `Invisible Scene`
  (bind _returnvalue (`GameplayStatics.GetActorOfClass` "/Script/LevelSequence.LevelSequenceActor"))
  (`LevelSequenceActor.SetSequence` _returnvalue "/Game/Sequences/InvisibleScreen.InvisibleScreen")
  (`MovieSceneSequencePlayer.Play` (`LevelSequenceActor.SequencePlayer` _returnvalue)))

(fn `Load Exemplars`
  (`BPFL_FileIO.LoadFileToStringArray` ""))

(fn `Select Cue Word from Exemplar Types`
  (returns (`Cue Word` :type String))
  (locals (`Cue Word List` :type "Array of String"))
  (bind _cue_word_list (`local.Cue Word List`))
  (bind _enumvalue (foreach `/Game/Scripts/ExemplarTypes` false)
    (:`LoopBody`
      (`KismetArrayLibrary.Array_Add` (`local.Cue Word List`) (`|GetEnumeratorNameAsString` _enumvalue)))
    (:`then`
      (return (`|GetArrayItem` _cue_word_list (`KismetMathLibrary.RandomInteger` (`KismetArrayLibrary.Array_Length` _cue_word_list)))))))

(fn `Set Up Experiment`
  (params (Type :type "/Game/Scripts/ExperimentType Enum" :default "NewEnumerator0"))
  (locals (`Exp Type` :type Integer))
  (switch `/Game/Scripts/ExperimentType` Type
    (:`NewEnumerator0`
      (set `self.Experiment ID` 1))
    (:`NewEnumerator1`
      (set `self.Experiment ID` 2)))
  (bind _asvruser (cast `/Game/Blueprints/Players/VRUser` (`GameplayStatics.GetPlayerPawn` 0)))
  (bind _gameinstance (`/Game/Blueprints/Players/VRUser.GameInstance` _asvruser))
  ;[0.003037 0.4983 0.02799 0.5 14] Generate new Save Slot Name and File Name
  (set `/Game/Blueprints/Players/GI_Experiments.Experiment Type` (`self.Experiment ID`) _gameinstance)
  (bind _save_slot_name (`/Game/Blueprints/Players/GI_Experiments.Generate Save Slot Name` _gameinstance))
  (`/Game/Blueprints/Players/GI_Experiments.Generate Exp File Name` _gameinstance)
  (`/Game/Blueprints/Players/VRUser.Save Session` _asvruser _save_slot_name))

(fn `Teleport`
  (switch `string` (`self.Target Room`)
    (:`Exemplar Room`
      (set `self.Target Room Transform` (`self.Exemplar Room Position`)))
    (:`Lobby Office`
      (set `self.Target Room Transform` (`self.Lobby Office Position`)))
    (:`Black Room`
      (set `self.Target Room Transform` (`self.Black Room Position`))))
  (bind _asvruser (cast `/Game/Blueprints/Players/VRUser` (`GameplayStatics.GetPlayerPawn` 0)))
  (`self.K2_SetActorLocation` _asvruser (`KismetMathLibrary.TransformLocation` (`self.Target Room Transform`)) false true))

(fn `UserConstructionScript`)

(fn `Visible Scene`
  (bind _returnvalue (`GameplayStatics.GetActorOfClass` "/Script/LevelSequence.LevelSequenceActor"))
  (`LevelSequenceActor.SetSequence` _returnvalue "/Game/Sequences/VisibleScreen.VisibleScreen")
  (`MovieSceneSequencePlayer.Play` (`LevelSequenceActor.SequencePlayer` _returnvalue)))