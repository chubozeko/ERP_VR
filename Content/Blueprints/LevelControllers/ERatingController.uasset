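; Level controller for the VR experiment's rating scene, where the user picks an exemplar category and rates it.
; It loads the VRUser session, fades in after a configured delay, and switches menu pages by teleporting MenuPanel.
; ExecuteButtonFunction routes ScreenButtons to category selection, rating save with trial-index-dependent completion or CSV export, or the next trial level.
; Fades swap Level Sequences; the gaze-based button polling here is disconnected.
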(event `self.ReceiveBeginPlay`
  (`self.Invisible Scene`)
  (`KismetSystemLibrary.Delay` 0.2)
  (bind _asvruser (cast `/Game/Blueprints/Players/VRUser` (`GameplayStatics.GetPlayerPawn` 0)))
  (bind _output_get (set `self.As VRUser` _asvruser))
  (bind _gameinstance (`/Game/Blueprints/Players/VRUser.GameInstance` _output_get))
  (`/Game/Blueprints/Players/VRUser.Load Session` _output_get self (`/Game/Blueprints/Players/GI_Experiments.Save Slot Name` _gameinstance))
  (`self.View Categories`)
  (bind _interval_in_seconds (`self.Convert Interval to Seconds` (`/Game/Blueprints/Players/GI_Experiments.Fade Interval` _gameinstance))) ; Fade Interval
  (`KismetSystemLibrary.Delay` _interval_in_seconds)
  (`self.FadeIntoScene`)
  (`/Game/Blueprints/Players/VRUser.Set Motion Controller Visibility` (`self.As VRUser`) true))

(event `self.ReceiveTick`
  (params (DeltaSeconds :type "Float (single-precision)")))

(event `View Categories`
  ;[0.06663 0.05448 0.2918 0.749 14] View Categories
  (`self.K2_SetActorLocation` (`self.Menu Panel`) (400.0 1085.0 150.0) false true))

(event `View Ratings`
  ;[0.06667 0.0549 0.2902 0.749 14] View Ratings
  (`self.K2_SetActorLocation` (`self.Menu Panel`) (0.0 1085.0 150.0) false true))

(event `Continue to Next Trial`
  ;[0.06663 0.05448 0.2918 0.749 14] Continue to Next Exemplar
  (`self.FadeToBlack`)
  (`self.Invisible Scene`)
  (`GameplayStatics.OpenLevelBySoftObjectPtr` "/Game/Levels/Experiment_1.Experiment_1"))

(event `View Experiment Complete`
  ;[0.06663 0.05448 0.2918 0.749 14] View Experiment Complete
  (`self.K2_SetActorLocation` (`self.Menu Panel`) (-400.0 1085.0 150.0) false true))

(event `Finish Session`
  ;[0.06663 0.05448 0.2918 0.749 14] Finish Session and Return to Lobby Office
  (`self.FadeToBlack`)
  (`self.Invisible Scene`)
  (`GameplayStatics.OpenLevelBySoftObjectPtr` "/Game/Levels/Home.Home"))

(fn `Convert Interval to Seconds`
  (params (`Interval in Milliseconds` :type "Float (double-precision)"))
  (returns (`Interval in Seconds` :type "Float (double-precision)"))
  (return (`KismetMathLibrary.Conv_IntToDouble` (/ `Interval in Milliseconds` 1000))))

(fn `Execute Button Function`
  (params (Button :type "/Game/Blueprints/ScreenButton Object Reference"))
  (bind _as_vruser (`self.As VRUser`))
  (bind _gameinstance (`/Game/Blueprints/Players/VRUser.GameInstance` _as_vruser))
  (switch `string` (`/Game/Blueprints/ScreenButton.Button Function` Button)
    (:`Beach`
      (set `self.Selected Category` (`/Game/Blueprints/ScreenButton.Exemplar Category` Button) :!label _label)
      (`self.View Ratings`))
    (:`Office`
      (goto _label))
    (:`CityStreet`
      (goto _label))
    (:`Highway`
      (goto _label))
    (:`Mountain`
      (goto _label))
    (:`Forest`
      (goto _label))
    (:`Rating`
      (set `self.Rating` (`/Game/Blueprints/ScreenButton.Rating Value` Button))
      (`/Game/Blueprints/Players/VRUser.Save Session` _as_vruser (`/Game/Blueprints/Players/GI_Experiments.Save Slot Name` _gameinstance))
      (switch `int` (`self.Current Trial Index`)
        (:`Default`
          (`self.View Experiment Complete`))
        (:`0`
          (bind _assave_experiments (cast `/Game/Blueprints/Players/Save_Experiments` (`/Game/Blueprints/Players/VRUser.Save REF` _as_vruser)))
          (`/Game/Blueprints/Players/Save_Experiments.Save Trials to CSV` _assave_experiments (`/Game/Blueprints/Players/GI_Experiments.Experiment File Name` _gameinstance))
          (`self.Finish Session`))))
    (:`ContinueToNextTrial`
      (`self.Continue to Next Trial`))))

(fn `FadeIntoScene`
  (bind _returnvalue (`GameplayStatics.GetActorOfClass` "/Script/LevelSequence.LevelSequenceActor"))
  (`LevelSequenceActor.SetSequence` _returnvalue "/Game/Sequences/FadeIn.FadeIn")
  (`MovieSceneSequencePlayer.Play` (`LevelSequenceActor.SequencePlayer` _returnvalue)))

(fn `FadeToBlack`
  (bind _returnvalue (`GameplayStatics.GetActorOfClass` "/Script/LevelSequence.LevelSequenceActor"))
  (`LevelSequenceActor.SetSequence` _returnvalue "/Game/Sequences/FadeOut.FadeOut")
  (`MovieSceneSequencePlayer.Play` (`LevelSequenceActor.SequencePlayer` _returnvalue)))

(fn `Get Article for Word`
  (params (Word :type String))
  (returns (`Correct Article` :type String))
  (locals (`Article to Use` :type String))
  (if (`KismetStringLibrary.Contains` "AEIOU" (`|GetArrayItem` (`KismetStringLibrary.GetCharacterArrayFromString` Word)))
    (set `local.Article to Use` "an")
    (else
      (set `local.Article to Use` "a")))
  (return (`local.Article to Use`)))

(fn `Get Object Looking At As ScreenButton`
  (returns (`ScreenButton Object` :type "/Game/Blueprints/ScreenButton Object Reference"))
  (bind _asvruser (cast `/Game/Blueprints/Players/VRUser` (`GameplayStatics.GetPlayerPawn` 0)))
  (bind _asscreen_button (cast `/Game/Blueprints/ScreenButton` (`/Game/Blueprints/Players/VRUser.Object Looking At` _asvruser)))
  (return _asscreen_button))

(fn `Invisible Scene`
  (bind _returnvalue (`GameplayStatics.GetActorOfClass` "/Script/LevelSequence.LevelSequenceActor"))
  (`LevelSequenceActor.SetSequence` _returnvalue "/Game/Sequences/InvisibleScreen.InvisibleScreen")
  (`MovieSceneSequencePlayer.Play` (`LevelSequenceActor.SequencePlayer` _returnvalue)))

(fn `UserConstructionScript`)

(fn `Visible Scene`
  (bind _returnvalue (`GameplayStatics.GetActorOfClass` "/Script/LevelSequence.LevelSequenceActor"))
  (`LevelSequenceActor.SetSequence` _returnvalue "/Game/Sequences/VisibleScreen.VisibleScreen")
  (`MovieSceneSequencePlayer.Play` (`LevelSequenceActor.SequencePlayer` _returnvalue)))