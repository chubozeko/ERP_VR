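; ETrial is a data record for one trial of a two-experiment study, holding the exemplar shown and the participant's response.
; InitializeTrial stores the trial number, exemplar name and type, and experiment ID, keeping the cue word only for Experiment 2.
; SaveResponses records the response and derives response time by subtracting timestamp components; both setters return self.
; PrintETrial returns a summary string of the setup fields, omitting response data.
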(fn `Calculate Response Time`
  (bind (_year _month _day _hour _minute _second _millisecond) (`KismetMathLibrary.BreakDateTime` (`self.Response Start Time`)))
  (bind (_year_2 _month_2 _day_2 _hour_2 _minute_2 _second_2 _millisecond_2) (`KismetMathLibrary.BreakDateTime` (`self.Response End Time`)))
  (set `self.Response Time` (`KismetMathLibrary.MakeTimespan` 0 (- _hour_2 _hour) (- _minute_2 _minute) (- _second_2 _second) (- _millisecond_2 _millisecond))))

(fn `Initialize Trial`
  (params (`Trial Number` :type Integer) (Exemplar :type "/Game/Blueprints/ExemplarObject Object Reference") (`Experiment Type` :type "/Game/Scripts/ExperimentType Enum" :default "NewEnumerator0") (`Cue Word` :type String))
  (returns (Trial :type "/Game/Blueprints/ETrial Object Reference"))
  (set `self.Trial Number` `Trial Number`)
  (bind _exemplar_name (`/Game/Blueprints/ExemplarObject.Get Exemplar Name` Exemplar))
  (set `self.Exemplar Name` _exemplar_name)
  (set `self.Exemplar Type` (`|GetEnumeratorNameAsString` (`/Game/Blueprints/ExemplarObject.Exemplar Type` Exemplar)))
  (switch `/Game/Scripts/ExperimentType` `Experiment Type`
    (:`NewEnumerator0`
      (set `self.Experiment ID` 1))
    (:`NewEnumerator1`
      (set `self.Experiment ID` 2)
      (set `self.Cue Word` `Cue Word`)))
  (return self))

(fn `Print ETrial`
  (returns (`ETrial toString` :type String))
  (return (`KismetStringLibrary.Concat_StrStr` "Trial Nr: " (`KismetStringLibrary.Conv_IntToString` (`self.Trial Number`)) "; Exp Id: " (`KismetStringLibrary.Conv_IntToString` (`self.Experiment ID`)) "; Exemplar Name: " (`self.Exemplar Name`) "; Exemplar Type: " (`self.Exemplar Type`) "; Cue Word: " (`self.Cue Word`))))

(fn `Save Responses`
  (params (Response :type String) (`Response Start Time` :type "DateTime Structure") (`Response End Time` :type "DateTime Structure"))
  (returns (Trial :type "/Game/Blueprints/ETrial Object Reference"))
  (set `self.Response` Response)
  (set `self.Response Start Time` `Response Start Time`)
  (set `self.Response End Time` `Response End Time`)
  (`self.Calculate Response Time`)
  (return self))