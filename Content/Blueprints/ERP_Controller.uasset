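; Controller for an ERP experiment app that runs the in-world menu and launches Experiment 1 or 2.
; Tick polls the character's looked-at ScreenButton and, when selected, switches menus, quits or starts an experiment.
; Starting one spawns trials from shuffled exemplars (Experiment 2 adds random cue words), saves the session to a new slot and opens its level.
; Also holds room-teleport and sequence-fade helpers; session loading is unwired.
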(event `self.ReceiveBeginPlay`
  (`self.ShowMainMenu`))

(event `self.ReceiveTick`
  (params (DeltaSeconds :type "Float (single-precision)"))
  ;[0 0.3763 0.02029 0.502 14] Check for Object being Looked at
  (for _array_element (`self.Main Menu Buttons`)
    (bind _screenbutton_object (`self.Get Object Looking At As ScreenButton`))
    (if (and (== _screenbutton_object _array_element) (`/Game/Blueprints/ScreenButton.IsSelected` _array_element))
      (`self.Execute Button Function` _array_element)
      (set `/Game/Blueprints/ScreenButton.IsSelected` false _array_element)))
  (for _array_element_2 (`self.Experiments Buttons`)
    (bind _screenbutton_object_2 (`self.Get Object Looking At As ScreenButton`))
    (if (and (== _screenbutton_object_2 _array_element_2) (`/Game/Blueprints/ScreenButton.IsSelected` _array_element_2))
      (`self.Execute Button Function` _array_element_2)
      (set `/Game/Blueprints/ScreenButton.IsSelected` false _array_element_2)))
  (for _array_element_3 (`self.Change Avatar Buttons`)
    (bind _screenbutton_object_3 (`self.Get Object Looking At As ScreenButton`))
    (if (and (== _screenbutton_object_3 _array_element_3) (`/Game/Blueprints/ScreenButton.IsSelected` _array_element_3))
      (`self.Execute Button Function` _array_element_3)
      (set `/Game/Blueprints/ScreenButton.IsSelected` false _array_element_3))))

(fn `Convert Interval to Seconds`
  (params (`Interval in Milliseconds` :type "Float (double-precision)"))
  (returns (`Interval in Seconds` :type "Float (double-precision)"))
  (return (`KismetMathLibrary.Conv_IntToDouble` (/ `Interval in Milliseconds` 1000))))

(fn `Execute Button Function`
  (params (Button :type "/Game/Blueprints/ScreenButton Object Reference"))
  (switch `string` (`/Game/Blueprints/ScreenButton.Button Function` Button)
    (:`Experiments`
      (`self.ShowExperimentsMenu`))
    (:`Exp1`
      (`self.Initialize Experiment 1 Trials`)
      (`self.Set Up Experiment` "NewEnumerator0")
      (`GameplayStatics.OpenLevelBySoftObjectPtr` "/Game/Levels/Experiment_1.Experiment_1"))
    (:`Exp2`
      (`self.Initialize Experiment 2 Trials`)
      (`self.Set Up Experiment` "NewEnumerator1")
      (`GameplayStatics.OpenLevelBySoftObjectPtr` "/Game/Levels/Experiment_2.Experiment_2"))
    (:`ChangeAvatar`
      (`self.ShowChangeAvatarMenu`)
      (`KismetSystemLibrary.PrintString` "You want to change your Avatar" true false))
    (:`BackToMain`
      (`self.ShowMainMenu`))
    (:`Quit`
      (`KismetSystemLibrary.QuitGame` null "Quit"))))

(fn `FadeIntoScene`
  (bind _returnvalue (`GameplayStatics.GetActorOfClass` "/Script/LevelSequence.LevelSequenceActor"))
  (`LevelSequenceActor.SetSequence` _returnvalue "/Game/Sequences/FadeIn.FadeIn")
  (`MovieSceneSequencePlayer.Play` (`LevelSequenceActor.SequencePlayer` _returnvalue)))

(fn `FadeToBlack`
  (bind _returnvalue (`GameplayStatics.GetActorOfClass` "/Script/LevelSequence.LevelSequenceActor"))
  (`LevelSequenceActor.SetSequence` _returnvalue "/Game/Sequences/FadeOut.FadeOut")
  (`MovieSceneSequencePlayer.Play` (`LevelSequenceActor.SequencePlayer` _returnvalue)))

(fn `Get Object Looking At As ScreenButton`
  (returns (`ScreenButton Object` :type "/Game/Blueprints/ScreenButton Object Reference"))
  (bind _asbp_fps_character (cast `/Game/Blueprints/BP_FPS_Character` (`GameplayStatics.GetPlayerCharacter` 0)))
  (bind _asscreen_button (cast `/Game/Blueprints/ScreenButton` (`/Game/Blueprints/BP_FPS_Character.ObjectLookingAt` _asbp_fps_character)))
  (return _asscreen_button))

(fn `Initialize Experiment 1 Trials`
  (bind _exemplars (`self.Exemplars`))
  (`KismetArrayLibrary.Array_Shuffle` _exemplars)
  (for (_array_element _array_index) _exemplars
    (bind _returnvalue (`|SpawnActorFromClass` "/Game/Blueprints/ExperimentTrial.ExperimentTrial_C" (`self.GetTransform` self) "Undefined" "OverrideRootScale" null null))
    (bind _trial (`/Game/Blueprints/ExperimentTrial.Initialize Trial` _returnvalue _array_index _array_element "NewEnumerator0" ""))
    (`KismetArrayLibrary.Array_Add` (`self.Experiment 1 Trials`) _trial)))

(fn `Initialize Experiment 2 Trials`
  (locals (`Cue Word List` :type "Array of String"))
  (bind _exemplars (`self.Exemplars`))
  (bind _cue_word_list (`local.Cue Word List`))
  (`KismetArrayLibrary.Array_Shuffle` _exemplars)
  (for (_array_element _array_index) _exemplars
    (bind _returnvalue (`|SpawnActorFromClass` "/Game/Blueprints/ExperimentTrial.ExperimentTrial_C" (`self.GetTransform` self) "Undefined" "OverrideRootScale" null null))
    (bind _enumvalue (foreach `/Game/Scripts/ExemplarTypes` false)
      (:`LoopBody`
        (`KismetArrayLibrary.Array_Add` _cue_word_list (`|GetEnumeratorNameAsString` _enumvalue)))
      (:`then`
        (bind _trial (`/Game/Blueprints/ExperimentTrial.Initialize Trial` _returnvalue _array_index _array_element "NewEnumerator1" (`|GetArrayItem` _cue_word_list (`KismetMathLibrary.RandomInteger` (`KismetArrayLibrary.Array_Length` _cue_word_list)))))
        (`KismetArrayLibrary.Array_Add` (`self.Experiment 2 Trials`) _trial)))))

(fn `Set Up Experiment`
  (params (Type :type "/Game/Scripts/ExperimentType Enum" :default "NewEnumerator0"))
  (locals (`Exp Type` :type Integer))
  (switch `/Game/Scripts/ExperimentType` Type
    (:`NewEnumerator0`
      (set `self.Experiment ID` 1))
    (:`NewEnumerator1`
      (set `self.Experiment ID` 2)))
  (bind _asbp_fps_character (cast `/Game/Blueprints/BP_FPS_Character` (`GameplayStatics.GetPlayerCharacter` 0)))
  (bind _gameinstance (`/Game/Blueprints/BP_FPS_Character.GameInstance` _asbp_fps_character))
  ;[0.003037 0.4983 0.02799 0.5 14] Generate new Save Slot Name
  (set `/Game/Blueprints/GI_Experiments.Experiment Type` (`self.Experiment ID`) _gameinstance)
  (bind _save_slot_name (`/Game/Blueprints/GI_Experiments.Generate Save Slot Name` _gameinstance))
  (`/Game/Blueprints/BP_FPS_Character.Save Session` _asbp_fps_character _save_slot_name))

(fn `ShowChangeAvatarMenu`
  (`self.K2_SetActorLocation` (`self.Menu Panel`) (-120.0 685.0 150.0) false false))

(fn `ShowExperimentsMenu`
  (`self.K2_SetActorLocation` (`self.Menu Panel`) (120.0 685.0 150.0) false false)
  (for _array_element (`self.Main Menu Buttons`)
    (`self.SetActorHiddenInGame` _array_element true)
    (`SceneComponent.SetVisibility` (`/Game/Blueprints/Master_Interact.DefaultSceneRoot` _array_element) false false))
  (for _array_element_2 (`self.Experiments Buttons`)
    (`self.SetActorHiddenInGame` _array_element_2 false)
    (`SceneComponent.SetVisibility` (`/Game/Blueprints/Master_Interact.DefaultSceneRoot` _array_element_2) false false)))

(fn `ShowMainMenu`
  (`self.K2_SetActorLocation` (`self.Menu Panel`) (0.0 685.0 150.0) false false)
  (for _array_element (`self.Main Menu Buttons`)
    (`self.SetActorHiddenInGame` _array_element false)
    (`SceneComponent.SetVisibility` (`/Game/Blueprints/Master_Interact.DefaultSceneRoot` _array_element) false false))
  (for _array_element_2 (`self.Experiments Buttons`)
    (`self.SetActorHiddenInGame` _array_element_2 true)
    (`SceneComponent.SetVisibility` (`/Game/Blueprints/Master_Interact.DefaultSceneRoot` _array_element_2) false false)))

(fn `Teleport`
  (switch `string` (`self.Target Room`)
    (:`Exemplar Room`
      (set `self.Target Room Transform` (`self.Exemplar Room Position`)))
    (:`Lobby Office`
      (set `self.Target Room Transform` (`self.Lobby Office Position`)))
    (:`Black Room`
      (set `self.Target Room Transform` (`self.Black Room Position`))))
  (bind _asbp_fps_character (cast `/Game/Blueprints/BP_FPS_Character` (`GameplayStatics.GetPlayerCharacter` 0)))
  (`self.K2_SetActorLocation` _asbp_fps_character (`KismetMathLibrary.TransformLocation` (`self.Target Room Transform`)) false true)
  (`/Game/Blueprints/BP_FPS_Character.Unset Room Movement` _asbp_fps_character))

(fn `Teleport to Black Room`
  (bind _asbp_fps_character (cast `/Game/Blueprints/BP_FPS_Character` (`GameplayStatics.GetPlayerCharacter` 0)))
  (`self.K2_SetActorLocation` _asbp_fps_character (`KismetMathLibrary.TransformLocation` (`self.Black Room Position`)) false true)
  (`/Game/Blueprints/BP_FPS_Character.Unset Room Movement` _asbp_fps_character))

(fn `Teleport to Exemplar Room`
  (bind _asbp_fps_character (cast `/Game/Blueprints/BP_FPS_Character` (`GameplayStatics.GetPlayerCharacter` 0)))
  (`self.K2_SetActorLocation` _asbp_fps_character (`KismetMathLibrary.TransformLocation` (`self.Exemplar Room Position`)) false true)
  (`/Game/Blueprints/BP_FPS_Character.Unset Room Movement` _asbp_fps_character))

(fn `Teleport to Lobby Office`
  (bind _asbp_fps_character (cast `/Game/Blueprints/BP_FPS_Character` (`GameplayStatics.GetPlayerCharacter` 0)))
  (`self.K2_SetActorLocation` _asbp_fps_character (`KismetMathLibrary.TransformLocation` (`self.Lobby Office Position`)) false true)
  (`/Game/Blueprints/BP_FPS_Character.Unset Room Movement` _asbp_fps_character))

(fn `UserConstructionScript`)